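; Interactable poster stand for a poster puzzle, displaying a swappable poster texture and reporting its index to a PuzzleChecker on interaction.
; Selection toggles the ceiling lamp material and fades the spotlight via a timeline.
; A dynamic material instance created in the construction script drives the poster image.
; On puzzle completion, it destroys its interaction widget and adds a junk required key, apparently to block further use.
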(event Custom|SetNewPoster
  (params (Texture :type Texture%20Object%20Reference) (PosterIndex :type Integer))
  (Rendering|Material|SetTextureParameterValue (Variables|Default|GetDynamicPosterMaterial) "PosterTexture" Texture)
  (Variables|Default|SetPosterTexture Texture)
  (Variables|Default|SetPoster%20Index PosterIndex))

(event Custom|OnPuzzleCompleted
  (Components|DestroyComponent (Variables|Default|GetAC_InteractableWidget))
  (Utilities|Array|Add (Variables|Default|GetKeys%20Required%20to%20Use) "appdatapornomuerte12312313131312313"))

(event Custom|ToggleSelected
  (params (NowSelected :type Boolean))
  (Rendering|Material|SetMaterial (Variables|Default|GetSM_lamparadetecho) 1 (select NowSelected "/Game/Levels/_GENERATED/notic/M_CeilingLight_Inst1.M_CeilingLight_Inst1" "/Game/modelos/Bath_Hygiene/Material/Metal_04_Mat.Metal_04_Mat"))
  (if NowSelected
    (bind _newtrack_0 (Timeline|Timeline PlayFromStart)
      (:Update
        (Rendering|Components|Light|SetIntensity (Variables|Default|GetSpotLight) (Math|Float|Lerp 0.0 (Variables|Default|GetIntensity) _newtrack_0))))
    (else
      (Timeline|Timeline ReverseFromEnd))))

(event EventBeginPlay
  (Variables|Default|SetIntensity (Variables|/Script/Engine.LightComponentBase|GetIntensity (Variables|Default|GetSpotLight)))
  (CallFunction|ToggleSelected false)
  (Rendering|Material|SetMaterial (Variables|Default|GetStand) 0 (Variables|Default|GetMaterial)))

(event EventOnSelect
  (params (Type :type Integer))
  (bind _ac_interactablewidget (Variables|Default|GetAC_InteractableWidget)
    (:then
      (Default|Update _ac_interactablewidget Type))
    (:else)))

(event EventOnDeselect
  (bind _ac_interactablewidget (Variables|Default|GetAC_InteractableWidget)
    (:then
      (Default|Hide _ac_interactablewidget))
    (:else)))

(event EventInteract
  (Default|SelectPoster (Variables|Default|GetPuzzle%20Checker) (Variables|Default|GetIndex)))

(fn ConstructionScript
  (bind _poster (Variables|Default|GetPoster))
  (Rendering|Material|SetMaterial (Variables|Default|GetCartelAtril) 0 (Variables|Default|GetMaterialCartel))
  (Rendering|Material|SetMaterial (Variables|Default|GetStand) 0 (Variables|Default|GetMaterial))
  (Variables|Default|GetDynamicPosterMaterial
    (:then
      (Rendering|Material|SetTextureParameterValue (Variables|Default|GetDynamicPosterMaterial) "PosterTexture" (Variables|Default|GetPosterTexture)))
    (:else
      (bind _returnvalue (Rendering|Material|CreateDynamicMaterialInstance _poster 0 (Rendering|Material|GetMaterial _poster 0) "None" :!class /Script/Engine.PrimitiveComponent))
      (Variables|Default|SetDynamicPosterMaterial _returnvalue)
      (Rendering|Material|SetMaterial (Variables|Default|GetPoster) 0 _returnvalue))))

(fn FInitialize
  (params (Index :type Integer) (PuzzleChecker :type BP%20Posters%20Puzzle%20Checker%20PE%20Invoker%20Object%20Reference))
  (Variables|Default|SetIndex Index)
  (Variables|Default|SetPuzzle%20Checker PuzzleChecker)
  (Variables|Default|SetPoster%20Index Index))

(fn KeysRequiredtoUse
  (return (Variables|Default|GetKeys%20Required%20to%20Use)))