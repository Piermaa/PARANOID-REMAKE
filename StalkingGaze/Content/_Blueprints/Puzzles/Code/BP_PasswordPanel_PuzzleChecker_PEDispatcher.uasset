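; Keypad password panel puzzle checker that collects button codes into a dash-padded display and submits them to its parent's solution check.
; Special codes clear or submit, digits stop at the default code's length, and input is ignored once solved.
; Success shows OPEN; failure shows LOCK, restores dashes on a timer, and plays subtitle dialogue, either a wrong-order hint or an escalating fail line.
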(event Custom|ReceivePressedBtn
  (params (ButtonCode :type Integer))
  (Audio|PlaySound2D (Variables|Default|GetOnButtonPressSFX) 1.0 1.0 0.0 0 0 false)
  (if (not (Variables|Default|GetbIsSolved))
    (switch int ButtonCode
      (:Default
        (if (not (> (Utilities|String|Len (Variables|Default|GetCurrentPassword)) (- (Utilities|String|Len (Variables|Default|GetDefaultPasswordCode)) 1)))
          (bind _output_get (Variables|Default|SetCurrentPassword (Utilities|String|Append (Variables|Default|GetCurrentPassword) (Utilities|String|ToString(Integer) ButtonCode))))
          (CallFunction|FUpdateText _output_get)
          (if (Utilities|Time|IsValidTimerHandle (Variables|Default|GetRestoringTimerHandle)) :!label _label
            (Utilities|Time|ClearandInvalidateTimerbyHandle (Variables|Default|GetRestoringTimerHandle)))))
      (:-2
        (Variables|Default|SetCurrentPassword "")
        (CallFunction|FUpdateText (Variables|Default|GetDefaultPasswordCode))
        (goto _label))
      (:-1
        (CallFunction|CheckPuzzleSolution (Variables|Default|GetCurrentPassword))))))

(event Custom|RestoreDefaultText
  (CallFunction|FUpdateText "----"))

(event EventOnPuzzleUnsolved
  (|CallParentFunction)
  (Audio|PlaySound2D (Variables|Default|GetOnPasswordWrongSFX) 1.0 1.0 0.0 0 0 false)
  (Utilities|FlowControl|Sequence
    (:then_0
      (CallFunction|FUpdateText "LOCK")
      (bind _aspc_first_person_controller (Utilities|Casting|CastToPC_FirstPersonController (Game|GetPlayerController 0)))
      (if (CallFunction|FCheckPasswordIsCorrectButOrderIsWrong (Variables|Default|GetCurrentPassword))
        (Default|SetNewDialogue (Variables|/Game/_Blueprints/Widgets/WBP_HUD.WBP_HUD_C|GetWBP_SubtitlesMaster (Variables|/Game/_Blueprints/Controller/PC_FirstPersonController.PC_FirstPersonController_C|GetHUD%20Widget _aspc_first_person_controller)) (CallFunction|GetDialogue (Utilities|Struct|BreakDataTableRowHandle (Variables|ParaniodEvents|GetCorrectNumbersWrongOrderDialogue))))
        (else
          (Default|SetNewDialogue (Variables|/Game/_Blueprints/Widgets/WBP_HUD.WBP_HUD_C|GetWBP_SubtitlesMaster (Variables|/Game/_Blueprints/Controller/PC_FirstPersonController.PC_FirstPersonController_C|GetHUD%20Widget _aspc_first_person_controller)) (CallFunction|GetDialogue (Utilities|Struct|BreakDataTableRowHandle (Utilities|Array|Get(acopy) (Variables|ParaniodEvents|GetFaildialogues) (Variables|Default|GetFailCount)))))
          (if (< (Variables|Default|GetFailCount) 2)
            (Math|Integer|IncrementInt (Variables|Default|GetFailCount))))))
    (:then_1
      (Variables|Default|SetCurrentPassword "")
      (bind _returnvalue (Utilities|Time|SetTimerbyEvent (delegate Custom|RestoreDefaultText) 2.0))
      (Variables|Default|SetRestoringTimerHandle _returnvalue))))

(event EventOnPuzzleSolved
  (|CallParentFunction)
  (CallFunction|FUpdateText "OPEN"))

(fn ConstructionScript
  (|CallParentFunction)
  (CallFunction|FUpdateText (Variables|Default|GetDefaultPasswordCode)))

(fn FUpdateText
  (params (NewText :type String))
  (LocalVariables|SetTempNewText NewText)
  (for _index (range 0 (- (- (Utilities|String|Len (Variables|Default|GetDefaultPasswordCode)) (Utilities|String|Len NewText)) 1))
    (LocalVariables|SetTempNewText (Utilities|String|Append (LocalVariables|GetTempNewText) "-")))
  (Rendering|Components|TextRender|SetText (Variables|Default|GetPasswordText) (Utilities|Text|ToText(String) (LocalVariables|GetTempNewText))))