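; Puzzle checker Blueprint that validates a submitted string solution and invokes paranoid events when the puzzle is solved.
; An exact match with PuzzleSolution calls OnPuzzleSolved, which tries to dispatch paranoid events and sets IsSolved; any mismatch calls OnPuzzleUnsolved, an empty hook for overrides.
; A helper function detects right-password-wrong-order attempts by testing that each solution character appears in the input, ignoring character counts and extra characters.
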(event Custom|CheckPuzzleSolution
  (params (SolutionAttempted :type String))
  (if (Utilities|Enum|Equal(Enum) SolutionAttempted (Variables|Default|GetPuzzleSolution))
    (CallFunction|OnPuzzleSolved)
    (else
      (CallFunction|OnPuzzleUnsolved))))

(event Custom|OnPuzzleSolved
  (Class|ParanoidEventDispatcher|TryDispatchParanoidEvents)
  (Variables|Default|SetbIsSolved true))

(event Custom|OnPuzzleUnsolved)

(fn ConstructionScript)

(fn FCheckPasswordIsCorrectButOrderIsWrong
  (params (PssToCheck :type String))
  (for _array_element (Utilities|String|GetCharacterArrayfromString (Variables|Default|GetPuzzleSolution))
    (if (not (Utilities|String|Contains PssToCheck _array_element))
      (return false)))
  (return true))