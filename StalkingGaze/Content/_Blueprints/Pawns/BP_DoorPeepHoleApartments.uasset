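; Possessable door peephole pawn, attached as a child to a door, that only allows use while that door is closed and not opening.
; On BeginPlay it caches the parent door and, if that is a BP_PeepHole_Door, copies its key settings, possess paranoid events and leave events.
; When the possession check fails, KeysRequiredToUse returns a deliberately nonexistent key name to block use, otherwise deferring to the parent class.
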(event EventBeginPlay
  (bind _returnvalue (Actor|GetAttachParentActor))
  (|CallParentFunction)
  (bind _asbp_door (Utilities|Casting|CastToBP_Door _returnvalue))
  (Variables|Default|SetOwning%20Door _asbp_door)
  (bind _asbp_peep_hole_door (Utilities|Casting|CastToBP_PeepHole_Door _returnvalue))
  (Variables|Default|SetKeysRequired (Variables|/Game/_Blueprints/Actors/Interactables/Doors/BP_PeepHole_Door.BP_PeepHole_Door_C|GetPeepHoleKeysRequired _asbp_peep_hole_door))
  (Variables|Default|SetConsumeKeys (Variables|/Game/_Blueprints/Actors/Interactables/Doors/BP_PeepHole_Door.BP_PeepHole_Door_C|GetPeepHoleConsumeKeys _asbp_peep_hole_door))
  (Variables|Default|SetKeysToUnlock (Variables|/Game/_Blueprints/Actors/Interactables/Doors/BP_PeepHole_Door.BP_PeepHole_Door_C|GetPeepHoleUnlockKeys _asbp_peep_hole_door))
  (Variables|Default|SetOnPossessParanoidEventsConsts (Variables|/Game/_Blueprints/Actors/Interactables/Doors/BP_PeepHole_Door.BP_PeepHole_Door_C|GetPeepHoleParanoidEventsConst _asbp_peep_hole_door))
  (Variables|Default|SetOnPossessParanoidEvents (Variables|/Game/_Blueprints/Actors/Interactables/Doors/BP_PeepHole_Door.BP_PeepHole_Door_C|GetPeepHoleParanoidEvents _asbp_peep_hole_door))
  (Variables|Default|SetOnPossessParanoidEventsNames (Variables|/Game/_Blueprints/Actors/Interactables/Doors/BP_PeepHole_Door.BP_PeepHole_Door_C|GetPeepHoleParanoidEventsNames _asbp_peep_hole_door))
  (Variables|Default|SetUnpossessEvent (Variables|/Game/_Blueprints/Actors/Interactables/Doors/BP_PeepHole_Door.BP_PeepHole_Door_C|GetOnPeepholeLeaveEvents _asbp_peep_hole_door)))

(fn ConstructionScript
  (|CallParentFunction))

(fn CheckIsPossessable
  (bind _owning_door (Variables|Default|GetOwning%20Door))
  (return (Math|Boolean|ANDBoolean (Variables|/Script/StalkingGaze.Door|GetbIsClosed _owning_door) (not (Variables|/Script/StalkingGaze.Door|GetbOpening _owning_door)) (|CallParentFunction))))

(fn KeysRequiredtoUse
  (if (CallFunction|CheckIsPossessable)
    (bind _keysrequiredtouse (|CallParentFunction))
    (return _keysrequiredtouse)
    (else
      (return (Utilities|Array|MakeArray "AAAAAAAAAAAAAAAAAAAAAAESTALLAVENOEXISTEEEEE")))))