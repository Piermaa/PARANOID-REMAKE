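; Possessable peephole pawn, by its name a chair variant, that attaches to a door and can only be possessed while that door is fully closed.
; On BeginPlay it caches the parent BP_Door and, if that is a BP_PeepHole_Door, copies the door's peephole key requirement, consumption and unlock settings.
; The possessable check reads the owning door's state, rejecting possession while it is open or opening.
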(event EventBeginPlay
  (bind _returnvalue (Actor|GetAttachParentActor))
  (|CallParentFunction)
  (bind _asbp_door (Utilities|Casting|CastToBP_Door _returnvalue))
  (Variables|Default|SetOwning%20Door _asbp_door)
  (bind _asbp_peep_hole_door (Utilities|Casting|CastToBP_PeepHole_Door _returnvalue))
  (Variables|Default|SetKeysRequired (Variables|/Game/_Blueprints/Actors/Interactables/Doors/BP_PeepHole_Door.BP_PeepHole_Door_C|GetPeepHoleKeysRequired _asbp_peep_hole_door))
  (Variables|Default|SetConsumeKeys (Variables|/Game/_Blueprints/Actors/Interactables/Doors/BP_PeepHole_Door.BP_PeepHole_Door_C|GetPeepHoleConsumeKeys _asbp_peep_hole_door))
  (Variables|Default|SetKeysToUnlock (Variables|/Game/_Blueprints/Actors/Interactables/Doors/BP_PeepHole_Door.BP_PeepHole_Door_C|GetPeepHoleUnlockKeys _asbp_peep_hole_door)))

(fn ConstructionScript
  (|CallParentFunction))

(fn CheckIsPossessable
  (bind _owning_door (Variables|Default|GetOwning%20Door))
  (return (and (Variables|/Script/ParanoidRemake.Door|GetbIsClosed _owning_door) (not (Variables|/Script/ParanoidRemake.Door|GetbOpening _owning_door)))))