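; Game instance for the Paranoid game that manages music playback and holds camera sensitivity and volume settings.
; PlayMusic fades out the active track and fades in a new 2D sound that persists across level transitions, with events to stop, pause and resume it.
; Sensitivity input is remapped by lerp, saved in GameConfig and broadcast through OnSensibilityChange.
; Volume values are stored in an array by ID.
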(event EventPlayMusic
  (params (Music :type Sound%20Base%20Object%20Reference) (FadeInTime :type Float%20%28double-precision%29) (FadeOutTime :type Float%20%28double-precision%29))
  (Variables|Default|GetActiveMP
    (:then
      (CallFunction|StopMusic FadeOutTime))
    (:else
      _))
  (bind _returnvalue (Audio|CreateSound2D Music 1.0 1.0 0.0 0 true))
  (bind _output_get (Variables|Default|SetActiveMP _returnvalue))
  (Audio|Components|Audio|FadeIn _output_get FadeInTime 1.0 0.0 "Linear" :!class /Script/Engine.AudioComponent))

(event EventStopMusic
  (params (FadeOutTime :type Float%20%28double-precision%29))
  (bind _activemp (Variables|Default|GetActiveMP)
    (:then
      (bind _output_get (Variables|Default|SetDyingMP _activemp))
      (Audio|Components|Audio|FadeOut _output_get FadeOutTime 0.0 "Linear" :!class /Script/Engine.AudioComponent))
    (:else)))

(event EventResume
  (Class|AudioComponent|SetPaused (Variables|Default|GetActiveMP) false))

(event EventPause
  (Class|AudioComponent|SetPaused (Variables|Default|GetActiveMP) true))

(fn FSetSensibility
  (params (Sensibility :type Float%20%28double-precision%29))
  (bind _returnvalue (Math|Float|Lerp 0.2 1.2 Sensibility))
  (bind _structout (Utilities|Struct|SetmembersinF_GameConfig (Variables|Default|GetGameConfig) _returnvalue))
  (Variables|Default|SetGameConfig _structout)
  (Default|CallOnSensibilityChange _returnvalue)
  (return))

(fn FSetVolume
  (params (Value :type Float%20%28double-precision%29) (ID :type Integer))
  (Utilities|Array|SetArrayElem (Variables|Default|GetVolumes) ID Value)
  (return true))