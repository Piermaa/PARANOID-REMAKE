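; Trigger volume for the Escopophobia chapter that overrides the player's camera shake while they are inside its box.
; On overlap by the player pawn, it passes its CameraShakeToPlay to the pawn's CameraShakeSelectorComponent as an override.
; When the pawn leaves, it clears that override.
; BeginPlay also draws a long-lived debug box showing the trigger bounds.
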(event OnComponentBeginOverlap(Box)
  (params (OverlappedComponent :type Primitive%20Component%20Object%20Reference) (OtherActor :type Actor%20Object%20Reference) (OtherComp :type Primitive%20Component%20Object%20Reference) (OtherBodyIndex :type Integer) (bFromSweep :type Boolean) (SweepResult :type Hit%20Result%20Structure%20%28by%20ref%29))
  (bind _returnvalue (Game|Player|GetPlayerPawn 0))
  (if (== OtherActor _returnvalue)
    (Class|CameraShakeSelectorComponent|SetOverrideCameraShake (Actor|GetComponentbyClass _returnvalue "/Script/ParanoidRemake.CameraShakeSelectorComponent") (Variables|CameraShake|GetCameraShakeToPlay))))

(event OnComponentEndOverlap(Box)
  (params (OverlappedComponent :type Primitive%20Component%20Object%20Reference) (OtherActor :type Actor%20Object%20Reference) (OtherComp :type Primitive%20Component%20Object%20Reference) (OtherBodyIndex :type Integer))
  (bind _returnvalue (Game|Player|GetPlayerPawn 0))
  (if (== OtherActor _returnvalue)
    (Class|CameraShakeSelectorComponent|ClearCameraShakeOverride (Actor|GetComponentbyClass _returnvalue "/Script/ParanoidRemake.CameraShakeSelectorComponent"))))

(event EventBeginPlay
  (Rendering|Debug|DrawDebugBox (Transformation|GetWorldLocation (Variables|Default|GetBox)) (Components|Box|GetScaledBoxExtent (Variables|Default|GetBox)) "(R=0.000000,G=0.859375,B=0.402766,A=1.000000)" "0, 0, 0" 1e+02 0.0))

(fn ConstructionScript)