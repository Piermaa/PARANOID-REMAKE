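; Elevator button for the Escopophobia chapter that sends its BP_Elevator to a set floor when interacted with.
; On BeginPlay it finds the owning elevator from its grandparent attach actor, falling back to its direct attach parent.
; Interact asks that elevator to move to the button's FloorNumber.
; The construction script applies optional custom mesh and materials and shows the floor number as toggleable text.
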(event EventBeginPlay
  (bind _asbp_elevator (Utilities|Casting|CastToBP_Elevator (Actor|GetAttachParentActor (Actor|GetAttachParentActor)))
    (:then
      (Variables|Default|SetElevatorOwner _asbp_elevator))
    (:CastFailed
      (Variables|Default|SetElevatorOwner (.AsBP%20Elevator (Utilities|Casting|CastToBP_Elevator (Actor|GetAttachParentActor)))))))

(event EventInteract
  (Default|TryMovetoFloor (Variables|Default|GetElevatorOwner) (Variables|Default|GetFloorNumber)))

(fn ConstructionScript
  (bind _custommesh (Variables|Default|GetCustomMesh))
  (for (_array_element _array_index) (Variables|Default|GetCustomMaterials)
    (Rendering|Material|SetMaterial (Variables|Default|GetButtonMesh) _array_index _array_element))
  (Rendering|SetVisibility (Variables|Default|GetTextRender) (Variables|Default|GetIsTextVisible) false)
  (Rendering|Components|TextRender|SetText (Variables|Default|GetTextRender) (Utilities|Text|ToText(Integer) (Variables|Default|GetFloorNumber)))
  (Utilities|IsValid _custommesh
    (:Is%20Valid
      (Components|StaticMesh|SetStaticMesh (Variables|Default|GetButtonMesh) _custommesh))))