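; Scripted elevator for the Escopophobia chapter that carries the player between floors marked by placed actors, with single-use floor buttons.
; Move requests close the doors if needed, then a timeline lerps the cabin's Z.
; Arrival updates the floor display, runs that floor's delayed door/travel events and invokes its Paranoid event batch.
; Global Paranoid events also drive the timeline-animated doors, while an invisible wall blocks passage until fully open.
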(event OnComponentBeginOverlap(Collision)
  (params (OverlappedComponent :type Primitive%20Component%20Object%20Reference) (OtherActor :type Actor%20Object%20Reference) (OtherComp :type Primitive%20Component%20Object%20Reference) (OtherBodyIndex :type Integer) (bFromSweep :type Boolean) (SweepResult :type Hit%20Result%20Structure%20%28by%20ref%29))
  (if (== OtherActor (Game|Player|GetPlayerPawn 0))
    (Variables|Default|SetbIsPlayerInside true)))

(event OnComponentEndOverlap(Collision)
  (params (OverlappedComponent :type Primitive%20Component%20Object%20Reference) (OtherActor :type Actor%20Object%20Reference) (OtherComp :type Primitive%20Component%20Object%20Reference) (OtherBodyIndex :type Integer))
  (if (== 0 (Game|Player|GetPlayerPawn 0))
    (Variables|Default|SetbIsPlayerInside false)))

(event Custom|CloseDoor
  ;[0.4456 0.9873 0.9948] Elevator
  ;;[1 1 1] DoorsAnimations
  (Audio|PlaySoundatLocation "/Game/Audio/SoundPresets/Elevator/MSP_SFX_Elevator_Close.MSP_SFX_Elevator_Close" (Transformation|GetActorLocation) "0, 0, 0" 1.0 1.0 0.0 "/Game/Audio/Attenuation/SAtt_Default.SAtt_Default" 0 0 0)
  (Variables|Default|SetisWorking true)
  (Variables|Default|SetDoorState "NewEnumerator3")
  (bind _track01 (Timeline|DoorsTimeline Reverse)
    (:Update
      (CallFunction|FLerpDoorPosition false _track01)
      (CallFunction|FLerpDoorPosition true _track01)
      (Collision|SetCollisionEnabled (Variables|Default|GetInvisibleWall) "QueryAndPhysics"))
    (:Finished
      (Variables|Default|SetisWorking false)
      (if (== _track01 0.0)
        (Variables|Default|SetDoorState "NewEnumerator1")
        (if (Variables|Default|GetMoveQueued)
          (Variables|Default|SetMoveQueued false)
          (CallFunction|StartMoving))
        (else
          (Variables|Default|SetDoorState "NewEnumerator0")
          (Collision|SetCollisionEnabled (Variables|Default|GetInvisibleWall) "NoCollision"))))))

(event Custom|OpenDoor
  ;[0.4456 0.9873 0.9948] Elevator
  ;;[1 1 1] DoorsAnimations
  (Audio|PlaySoundatLocation "/Game/Audio/SoundPresets/Elevator/MSP_SFX_Elevator_Open.MSP_SFX_Elevator_Open" (Transformation|GetActorLocation) "0, 0, 0" 1.0 1.0 0.0 "/Game/Audio/Attenuation/SAtt_Default.SAtt_Default" 0 0 0)
  (Variables|Default|SetisWorking true)
  (Variables|Default|SetDoorState "NewEnumerator2")
  (bind _track01 (Timeline|DoorsTimeline Play)
    (:Update
      (CallFunction|FLerpDoorPosition false _track01)
      (CallFunction|FLerpDoorPosition true _track01)
      (Collision|SetCollisionEnabled (Variables|Default|GetInvisibleWall) "QueryAndPhysics"))
    (:Finished
      (Variables|Default|SetisWorking false)
      (if (== _track01 0.0)
        (Variables|Default|SetDoorState "NewEnumerator1")
        (if (Variables|Default|GetMoveQueued)
          (Variables|Default|SetMoveQueued false)
          (CallFunction|StartMoving))
        (else
          (Variables|Default|SetDoorState "NewEnumerator0")
          (Collision|SetCollisionEnabled (Variables|Default|GetInvisibleWall) "NoCollision"))))))

(event Custom|GoToFloorWithDelay
  (params (Floor :type Integer) (Duration :type Float%20%28single-precision%29))
  ;[0.4456 0.9873 0.9948] Elevator
  (Utilities|FlowControl|Delay Duration)
  (CallFunction|MovetoFloor Floor))

(event Custom|MoveToFloor
  (params (Floor :type Integer))
  (bind _floorlocations (Variables|Elevator|GetFloorLocations))
  (bind (_value _returnvalue) (Utilities|Map|Find _floorlocations Floor))
  ;[0.4456 0.9873 0.9948] Elevator
  ;;[1 1 1] Move to Floor
  (if _returnvalue
    (Utilities|IsValid _value
      (:Is%20Valid
        (Variables|Default|SetCurrentFloorTarget (Transformation|GetActorLocation _value))
        (Variables|Default|SetCurrentFloorTargetIndex Floor)
        (Variables|Default|SetStartLocation (Transformation|GetActorLocation))
        (if (Utilities|Enum|Equal(Enum) (Variables|Default|GetDoorState) "NewEnumerator1")
          (CallFunction|StartMoving)
          (else
            (CallFunction|CloseDoor)
            (Variables|Default|SetMoveQueued true))))
      (:Is%20Not%20Valid
        ;;;[1 1 1] Ininputable soy ahora
        (Development|PrintString (Utilities|String|Append "Setea el actor del piso " (Utilities|String|ToString(Integer) Floor) " boludin") true true "(R=1.000000,G=0.014152,B=0.123819,A=1.000000)")))
    (else
      (Development|PrintString "Floor not defined" true true "(R=1.000000,G=0.000000,B=0.197169,A=1.000000)"))))

(event Custom|OpenDoorWithDelay
  (params (Open? :type Boolean) (Duration :type Float%20%28single-precision%29))
  ;[0.4456 0.9873 0.9948] Elevator
  (Utilities|FlowControl|Delay Duration)
  (if Open?
    (CallFunction|OpenDoor)
    (else
      (CallFunction|CloseDoor))))

(event Custom|Call%20Events
  (bind _floorevents (Variables|Elevator|GetFloorEvents))
  (bind _currentfloortargetindex (Variables|Default|GetCurrentFloorTargetIndex))
  (bind (_value _returnvalue) (Utilities|Map|Find _floorevents _currentfloortargetindex))
  (bind (_elevatorevents _paranoidevents) (Utilities|Struct|BreakF_FloorEvent _value))
  ;[0.4456 0.9873 0.9948] Elevator
  ;;[0.2128 0.07197 0.4531] Events
  (if _returnvalue
    (Rendering|Components|TextRender|SetText (Variables|Default|GetTextRender) (Utilities|Text|ToText(Integer) _currentfloortargetindex))
    (Audio|PlaySoundatLocation "/Game/Audio/SoundPresets/Elevator/MSP_SFX_Elevator_Button_Press.MSP_SFX_Elevator_Button_Press" (Transformation|GetActorLocation) "0, 0, 0" 1.0 1.0 0.0 "/Game/Audio/Attenuation/SAtt_Default.SAtt_Default" 0 0 0)
    (for _array_element _elevatorevents
      (switch Utilities|FlowControl|Switch|SwitchonE_ElevatorEventType (.EventType (Utilities|Struct|BreakF_ElevatorEvent _array_element))
        (:NewEnumerator1
          (Utilities|FlowControl|Delay (.AfterSeconds (Utilities|Struct|BreakF_ElevatorEvent _array_element)))
          (CallFunction|CloseDoor))
        (:NewEnumerator2
          (Utilities|FlowControl|Delay (.AfterSeconds (Utilities|Struct|BreakF_ElevatorEvent _array_element)))
          (CallFunction|OpenDoor))
        (:NewEnumerator12
          (CallFunction|GotoFloorwithDelay (.Floor (Utilities|Struct|BreakF_ElevatorEvent _array_element)) (.AfterSeconds (Utilities|Struct|BreakF_ElevatorEvent _array_element))))))
    (Class|ParanoidEventDispatcher|InvokeBatch (Variables|Default|GetDispatcherComponent) (.AsParanoid%20Game%20Instance (Utilities|Casting|CastToParanoidGameInstance (Game|GetGameInstance))) _paranoidevents)
    (else
      (Development|PrintString (Utilities|String|Append "Floor event not defined on " (Utilities|String|ToString(Integer) (Variables|Default|GetCurrentFloorTargetIndex)) " floor") true true "(R=1.000000,G=0.014152,B=0.123819,A=1.000000)"))))

(event Custom|TryMoveToFloor
  (params (Floor :type Integer))
  (if (Variables|Default|GetbIsPlayerInside)
    (if (Utilities|Set|Contains (Variables|Elevator|GetAvailableButtons) Floor)
      (Utilities|Set|Remove (Variables|Elevator|GetAvailableButtons) Floor)
      (if (not (Variables|Default|GetisWorking))
        (CallFunction|MovetoFloor Floor)
        (Audio|PlaySound2D "/Game/Audio/SoundPresets/Elevator/MSP_SFX_Elevator_Button_Press.MSP_SFX_Elevator_Button_Press" 1.0 1.0 0.0 0 0 false)))))

(event Custom|Event
  (params (ParanoidEventName :type Name))
  ;[0.4456 0.9873 0.9948] Elevator
  (switch name ParanoidEventName
    (:OpenElevator
      (CallFunction|OpenDoor))
    (:CloseElevator
      (CallFunction|CloseDoor))))

(event Custom|StartMoving
  (bind _returnvalue (Transformation|GetActorLocation))
  (bind (_x _y) (Math|Vector|BreakVector _returnvalue))
  (Audio|Components|Audio|Play (Variables|Default|GetAudio) 0.0)
  ;[0.4456 0.9873 0.9948] Elevator
  (Variables|Default|SetisWorking true)
  (bind _track01 (Timeline|Timeline PlayFromStart)
    (:Update
      (Transformation|SetActorLocation (Math|Vector|MakeVector _x _y (Math|Float|Lerp (.Z (Math|Vector|BreakVector (Variables|Default|GetStartLocation))) (.Z (Math|Vector|BreakVector (Variables|Default|GetCurrentFloorTarget))) _track01)) true false))
    (:Finished
      (CallFunction|CallEvents)
      (Class|AudioParameterControllerInterface|SetTriggerParameter(Message) (Variables|Default|GetAudio) "OnStop"))))

(event Custom|StopMoving
  (bind _returnvalue (Transformation|GetActorLocation))
  (bind (_x _y) (Math|Vector|BreakVector _returnvalue))
  ;[0.4456 0.9873 0.9948] Elevator
  (Variables|Default|SetisWorking false)
  (bind _track01 (Timeline|Timeline Stop)
    (:Update
      (Transformation|SetActorLocation (Math|Vector|MakeVector _x _y (Math|Float|Lerp (.Z (Math|Vector|BreakVector (Variables|Default|GetStartLocation))) (.Z (Math|Vector|BreakVector (Variables|Default|GetCurrentFloorTarget))) _track01)) true false))
    (:Finished
      (CallFunction|CallEvents)
      (Class|AudioParameterControllerInterface|SetTriggerParameter(Message) (Variables|Default|GetAudio) "OnStop"))))

(event EventBeginPlay
  ;[0.4456 0.9873 0.9948] Elevator
  (Utilities|FlowControl|Sequence
    (:then_0
      (bind _asparanoid_event_dispatcher (Utilities|Casting|CastToParanoidEventDispatcher (Variables|/Script/Engine.ChildActorComponent|GetChildActor (Variables|Default|GetPEDispatcherChild))))
      (Variables|Default|SetDispatcherComponent _asparanoid_event_dispatcher)
      (Collision|SetCollisionEnabled (Variables|Default|GetInvisibleWall) "NoCollision"))
    (:then_1
      (bind _asbp_paranoid_game_instance (Utilities|Casting|CastToBP_ParanoidGameInstance (Game|GetGameInstance)))
      (EventDispatchers|BindEventtoOnParanoidEvent _asbp_paranoid_game_instance (EventDispatchers|CreateEvent :!event Custom|Event)))))

(event EventPlayBlueprintAnimation
  (params (AnimationIndex :type Integer))
  ;[0.4456 0.9873 0.9948] Elevator
  ;;[1 1 1] DoorsAnimations
  (switch int AnimationIndex
    (:0
      (CallFunction|CloseDoor))
    (:1
      (CallFunction|OpenDoor))))

(fn ConstructionScript
  (|CallParentFunction)
  (Rendering|Components|TextRender|SetText (Variables|Default|GetTextRender) (Utilities|Text|ToText(Integer) (Variables|Elevator|GetDefaultFloor))))

(fn FLerpDoorPosition
  (params (IsLeft? :type Boolean) (Alpha :type Float%20%28single-precision%29))
  (LocalVariables|SetL_IsLeft IsLeft?)
  (Transformation|SetRelativeLocation (select (LocalVariables|GetL_IsLeft) (Variables|Default|GetDoorLeft) (Variables|Default|GetDoorRight)) (Math|Vector|Lerp(Vector) (Variables|/Script/Engine.SceneComponent|GetRelativeLocation (select (LocalVariables|GetL_IsLeft) (Variables|Default|GetCloseLocationLeft) (Variables|Default|GetCloseLocationRight))) (Variables|/Script/Engine.SceneComponent|GetRelativeLocation (select (LocalVariables|GetL_IsLeft) (Variables|Default|GetOpenLocationLeft) (Variables|Default|GetOpenLocationRight))) Alpha) false false)
  (return))