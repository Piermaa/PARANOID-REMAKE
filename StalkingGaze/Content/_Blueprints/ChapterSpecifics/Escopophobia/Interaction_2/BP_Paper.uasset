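; BP_Paper is an interactable paper prop in the Escopophobia chapter whose appearance changes with paranoid events.
; Its three interaction components start hidden, and each state change reveals the one selected by ParanoidEventsIndex, without hiding the others.
; Selection and deselection update or hide the interactable widget component.
; An unconnected branch for hiding components with a different index mapping never runs.
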(event EventBeginPlay
  (Rendering|SetVisibility (Variables|Default|GetInteraction1) false true)
  (Rendering|SetVisibility (Variables|Default|GetInteraction3) false true)
  (Rendering|SetVisibility (Variables|Default|GetInteraction2) false true))

(event EventOnSelect
  (params (Type :type Integer))
  (Default|Update (Variables|Default|GetAC_InteractableWidget) Type))

(event EventOnDeselect
  (Default|Hide (Variables|Default|GetAC_InteractableWidget)))

(event EventOnChangeState
  (bind _paranoideventsindex (Variables|Default|GetParanoidEventsIndex))
  (bind _interaction1 (Variables|Default|GetInteraction1))
  (bind _interaction3 (Variables|Default|GetInteraction3))
  (bind _interaction2 (Variables|Default|GetInteraction2))
  (bind _returnvalue (Utilities|Select :Index _paranoideventsindex :Option%200 _interaction1 :Option%201 _interaction2 :Option%202 _interaction3))
  (Utilities|IsValid _returnvalue
    (:Is%20Valid
      (Rendering|SetVisibility _returnvalue true true))))

(fn ConstructionScript
  (|CallParentFunction))