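; Staircase interaction for the Escopophobia chapter that removes mannequins once they are hidden from the player.
; While the player is inside the trigger box, a 0.2-second looping timer drives the check, which walks the mannequin array in reverse.
; For each mannequin under a height-difference threshold, a Camera-channel trace to the player ignores railings and mannequins, destroying that mannequin if something else blocks it.
; A debug key also starts the timer.
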(event OnComponentBeginOverlap(Box)
  (params (OverlappedComponent :type Primitive%20Component%20Object%20Reference) (OtherActor :type Actor%20Object%20Reference) (OtherComp :type Primitive%20Component%20Object%20Reference) (OtherBodyIndex :type Integer) (bFromSweep :type Boolean) (SweepResult :type Hit%20Result%20Structure%20%28by%20ref%29))
  (if (== OtherActor (Game|Player|GetPlayerPawn 0))
    (CallFunction|StartTimer)))

(event OnComponentEndOverlap(Box)
  (params (OverlappedComponent :type Primitive%20Component%20Object%20Reference) (OtherActor :type Actor%20Object%20Reference) (OtherComp :type Primitive%20Component%20Object%20Reference) (OtherBodyIndex :type Integer))
  (if (== OtherActor (Game|Player|GetPlayerPawn 0))
    (Utilities|Time|ClearandInvalidateTimerbyHandle (Variables|Default|GetCheckingTimer))))

(event Custom|CheckForDisable
  (bind (_arrayindex _arrayelement) (Utilities|Array|ReverseforEachLoop (Variables|Default|GetMannekins))
    (:LoopBody
      (Utilities|IsValid _arrayelement
        (:Is%20Valid
          (if (< (- (.Z (Math|Vector|BreakVector (Transformation|GetActorLocation _arrayelement))) (Utilities|PlayerLocation)) (Variables|Default|GetHeightDifference))
            (bind (_outhit _returnvalue) (Collision|LineTraceByChannel (+ (Transformation|GetActorLocation _arrayelement) "0.000000,0.000000,150.000000") (Transformation|GetActorLocation (Variables|Default|GetPlayerCharacter)) "TraceTypeQuery2" false (Variables|Default|GetAllActorsToIgnoreArray) "ForDuration" true "(R=1.000000,G=0.000000,B=0.000000,A=1.000000)" "(R=0.000000,G=1.000000,B=0.000000,A=1.000000)" 0.2))
            (if _returnvalue
              (if (not (== (.HitActor (Collision|BreakHitResult _outhit)) (Variables|Default|GetPlayerCharacter)))
                (Actor|DestroyActor _arrayelement)
                (Utilities|Array|RemoveIndex (Variables|Default|GetMannekins) _arrayindex)))))))))

(event Custom|Start%20Timer
  (bind _returnvalue (Utilities|Time|SetTimerbyEvent (EventDispatchers|CreateEvent :!event Custom|CheckForDisable) 0.2 true))
  (Variables|Default|SetCheckingTimer _returnvalue))

(event EventBeginPlay
  (bind _returnvalue (Game|GetPlayerCharacter 0))
  (Variables|Default|SetPlayerCharacter _returnvalue)
  (Variables|Default|SetCapsuleHeight (Variables|/Script/Engine.CapsuleComponent|GetCapsuleHalfHeight (Variables|/Script/Engine.Character|GetCapsuleComponent _returnvalue)))
  (Utilities|Array|AppendArray (Variables|Default|GetAllActorsToIgnoreArray) (Variables|Default|GetBarandas))
  (Utilities|Array|AppendArray (Variables|Default|GetAllActorsToIgnoreArray) (Variables|Default|GetMannekins)))

(event Input|KeyboardEvents|DebugKeyM
  (params (Key :type Key%20Structure :default "None") (ActionValue :type Input%20Action%20Value%20Structure))
  (:Pressed
    (CallFunction|StartTimer)))

(fn ConstructionScript)

(fn NewFunction)