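; Placard controller for the Escopophobia chapter's fifth interaction, driving a set of placard child actors during the wardrobes sequence.
; The construction script adds child actor components spaced along X and stores them in a struct array with per-placard timing and force settings.
; Wardrobes Start and End events from the Paranoid game instance start and stop a looping timer.
; Each child receives its settings on start, then elapsed time every tick of that timer.
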(event Custom|CountDown
  (for _array_element (Variables|Default|GetPlacardsStructs)
    (Class|BPIPlacards|FnTimeElapsed(Message) (Variables|/Script/Engine.ChildActorComponent|GetChildActor (Utilities|Struct|BreakF_Placard _array_element)) (Variables|Default|GetTime))))

(event Custom|Begin
  (for _array_element (Variables|Default|GetPlacardsStructs)
    (Class|BPIPlacards|FnInitialize(Message) (Variables|/Script/Engine.ChildActorComponent|GetChildActor (.Internal__ChildActor (Utilities|Struct|BreakF_Placard _array_element))) (.StartDelay (Utilities|Struct|BreakF_Placard _array_element)) (.LoopingTimeRange (Utilities|Struct|BreakF_Placard _array_element)) (.RandomForceRange (Utilities|Struct|BreakF_Placard _array_element))))
  (bind _returnvalue (Utilities|Time|SetTimerbyEvent (delegate Custom|CountDown) (Variables|Default|GetTime) true))
  (Variables|Default|SetTimerHandle _returnvalue))

(event Custom|Stop
  (Utilities|Time|ClearandInvalidateTimerbyHandle (Variables|Default|GetTimerHandle)))

(event Custom|Event
  (params (ParanoidEventName :type Name))
  (switch name ParanoidEventName
    (:WardrobesStart
      (CallFunction|Begin))
    (:WardrobesEnd
      (CallFunction|Stop))))

(event EventBeginPlay
  (bind _asbp_paranoid_game_instance (Utilities|Casting|CastToBP_ParanoidGameInstance (Game|GetGameInstance)))
  (EventDispatchers|BindEventtoOnParanoidEvent _asbp_paranoid_game_instance (EventDispatchers|CreateEvent :!event Custom|Event)))

(fn ConstructionScript
  (bind _placards (Variables|Default|GetPlacards))
  (bind _placardsstructs (Variables|Default|GetPlacardsStructs))
  (bind _returnvalue (- _placards 1))
  (Utilities|Array|Resize (Variables|Default|GetPlacardsStructs) _returnvalue)
  (for _index (range 0 _returnvalue)
    (bind _returnvalue_2 (AddComponent|AddChildActorComponent false (Math|Transform|MakeTransform (Math|Vector|MakeVector (Math|Conversions|ToFloat(Integer) (* _index 100)) 0.0 0.0))))
    (if (Utilities|Array|IsValidIndex _placardsstructs _index)
      (bind _structout (Utilities|Struct|SetmembersinF_Placard (Utilities|Array|Get(acopy) _placardsstructs _index) _returnvalue_2))
      (Utilities|Array|SetArrayElem (Variables|Default|GetPlacardsStructs) _index _structout)
      (Class|TestTypedElementInterfaceA|SetDisplayName(Message) _returnvalue_2 (Utilities|Struct|MakeScriptTypedElementHandle) "Mierdita" true))))