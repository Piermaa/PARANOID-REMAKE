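; BP_Door is an interactable door that a player or a matching named paranoid event can trigger, unless it is locked.
; It binds to the game instance's paranoid event dispatcher and, when the event name matches DoorName, interacts using the direction from the door to the player.
; The parent class handles the directional interaction, while a FlipFlop here alternates squeaky open and close sounds.
; Selection updates or hides the interactable widget.
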(event Custom|ParanoidEventListener
  (params (ParanoidEventName :type Name))
  (if (== (Variables|Door|GetDoorName) ParanoidEventName)
    (Class|DirectedInteractableInterface|DirectionDependantInteract (Math|Vector|GetUnitDirection(Vector) (Transformation|GetActorLocation) (Transformation|GetActorLocation (Game|Player|GetPlayerPawn 0))))))

(event EventOnSelect
  (params (Type :type Integer))
  (Default|Update (Variables|Default|GetAC_InteractableWidget) Type))

(event EventBeginPlay
  (|CallParentFunction)
  (bind _asbp_paranoid_game_instance (Utilities|Casting|CastToBP_ParanoidGameInstance (Game|GetGameInstance)))
  (EventDispatchers|BindEventtoOnParanoidEvent _asbp_paranoid_game_instance (EventDispatchers|CreateEvent :!event Custom|ParanoidEventListener)))

(event EventDirectionDependantInteract
  (params (Direction :type Vector :default "0, 0, 0"))
  (bind _returnvalue (Transformation|GetActorLocation))
  (if (not (Variables|Default|GetbIsLocked?))
    (|CallParentFunction Direction)
    (Utilities|FlowControl|FlipFlop
      (:A
        (Audio|PlaySoundatLocation "/Game/Audio/SoundPresets/Doors/MSP_SFX_Door_Open_Sqky.MSP_SFX_Door_Open_Sqky" _returnvalue "0, 0, 0" 1.0 1.0 0.0 "/Game/Audio/Attenuation/SAtt_Default.SAtt_Default" 0 0 0))
      (:B
        (Audio|PlaySoundatLocation "/Game/Audio/SoundPresets/Doors/MSP_SFX_Door_Close_Sqky.MSP_SFX_Door_Close_Sqky" _returnvalue "0, 0, 0" 1.0 1.0 0.0 "/Game/Audio/Attenuation/SAtt_Default.SAtt_Default" 0 0 0)))))

(event EventOnDeselect
  (Default|Hide (Variables|Default|GetAC_InteractableWidget)))

(fn ConstructionScript)