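; BP_FullWardrobeDoor_L is a left wardrobe door that reacts to the game instance's paranoid event matching its DoorName.
; PlayBlueprintAnimation either toggles a Timeline that lerps yaw between the starting rotation and MaxOpenDegrees, or, with PEUsesPhysics, enables physics and applies an angular impulse.
; The Timeline path ignores retriggers while moving and signals animation start and finish.
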(event Custom|CloseDoor
  (bind (_direction _newtrack_0) (Timeline|Timeline ReverseFromEnd)
    (:Update
      (Transformation|SetActorRotation (Math|Rotator|Lerp(Rotator) (Variables|Animation|GetStartRotation) (Variables|Animation|GetOpenRotation) _newtrack_0)))
    (:Finished
      (Variables|Animation|SetIsOpening false)
      (CallFunction|AnimationFinished (Utilities|Enum|Equal(Enum) _direction "Forward")))))

(event Custom|OpenDoor
  (bind (_direction _newtrack_0) (Timeline|Timeline PlayFromStart)
    (:Update
      (Transformation|SetActorRotation (Math|Rotator|Lerp(Rotator) (Variables|Animation|GetStartRotation) (Variables|Animation|GetOpenRotation) _newtrack_0)))
    (:Finished
      (Variables|Animation|SetIsOpening false)
      (CallFunction|AnimationFinished (Utilities|Enum|Equal(Enum) _direction "Forward")))))

(event Custom|ParanoidEventListener
  (params (ParanoidEventName :type Name))
  (if (== ParanoidEventName (Variables|ParanoidEvent|GetDoorName))
    (CallFunction|PlayBlueprintAnimation)))

(event EventPlayBlueprintAnimation
  (params (AnimationIndex :type Integer))
  (bind _static_mesh (Variables|Default|GetStatic%20Mesh))
  (if (Variables|ParanoidEvent|GetPEUsesPhysics)
    (Collision|SetCollisionResponsetoAllChannels _static_mesh "ECR_Ignore")
    (Collision|SetCollisionObjectType _static_mesh "ECC_PhysicsBody")
    (Collision|SetCollisionResponsetoChannel _static_mesh "ECC_WorldStatic" "ECR_Block")
    (Collision|SetCollisionEnabled _static_mesh "QueryAndPhysics")
    (Physics|SetSimulatePhysics _static_mesh true)
    (Class|PrimitiveComponent|AddAngularImpulseinDegrees _static_mesh (Math|Vector|MakeVector 0.0 0.0 (* (Variables|Animation|GetMaxOpenDegrees) 1e+01)) "None" true)
    (elif (not (Variables|Animation|GetIsOpening))
      (Variables|Animation|SetIsOpening true)
      (CallFunction|AnimationStarted)
      (bind _output_get (Variables|Default|SetAnimation%20Index (Math|Integer|SelectInt 1 0 (== (Variables|Default|GetAnimation%20Index) 0))))
      (switch int _output_get
        (:0
          (CallFunction|CloseDoor))
        (:1
          (CallFunction|OpenDoor))))))

(event EventBeginPlay
  (|CallParentFunction)
  (bind _output_get (Variables|Animation|SetStartRotation (Transformation|GetActorRotation)))
  (Variables|Animation|SetOpenRotation (Math|Rotator|MakeRotator (.Roll (Math|Rotator|BreakRotator _output_get)) (.Pitch (Math|Rotator|BreakRotator _output_get)) (Variables|Animation|GetMaxOpenDegrees)))
  (bind _asbp_paranoid_game_instance (Utilities|Casting|CastToBP_ParanoidGameInstance (Game|GetGameInstance)))
  (EventDispatchers|BindEventtoOnParanoidEvent _asbp_paranoid_game_instance (EventDispatchers|CreateEvent :!event Custom|ParanoidEventListener)))

(fn ConstructionScript
  (|CallParentFunction))