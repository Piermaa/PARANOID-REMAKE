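; Interactable bedside table drawer Blueprint that toggles between sliding open and closed.
; BeginPlay caches the start location and converts FinalLocation from a world-axis offset into an absolute target.
; PlayBlueprintAnimation flips AnimationIndex to play or reverse one Timeline, which lerps the whole actor between both locations.
; IsDrawing blocks retriggers mid-motion, and AnimationStarted and AnimationFinished report progress, the latter passing whether the Timeline ran forward.
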(event Custom|CloseDrawer
  (bind (_direction _newtrack_0) (Timeline|Timeline ReverseFromEnd)
    (:Update
      (Transformation|SetActorLocation (Math|Vector|Lerp(Vector) (Variables|Animation|GetStartLocation) (Variables|Animation|GetFinalLocation) _newtrack_0) false false))
    (:Finished
      (Variables|Animation|SetIsDrawing false)
      (CallFunction|AnimationFinished (Utilities|Enum|Equal(Enum) _direction "Forward")))))

(event Custom|OpenDrawer
  (bind (_direction _newtrack_0) (Timeline|Timeline PlayFromStart)
    (:Update
      (Transformation|SetActorLocation (Math|Vector|Lerp(Vector) (Variables|Animation|GetStartLocation) (Variables|Animation|GetFinalLocation) _newtrack_0) false false))
    (:Finished
      (Variables|Animation|SetIsDrawing false)
      (CallFunction|AnimationFinished (Utilities|Enum|Equal(Enum) _direction "Forward")))))

(event EventBeginPlay
  (bind _returnvalue (Transformation|GetActorLocation))
  (|CallParentFunction)
  (Variables|Animation|SetStartLocation _returnvalue)
  (Variables|Animation|SetFinalLocation (+ _returnvalue (Variables|Animation|GetFinalLocation))))

(event EventPlayBlueprintAnimation
  (params (AnimationIndex :type Integer))
  (if (not (Variables|Animation|GetIsDrawing))
    (CallFunction|AnimationStarted)
    (Variables|Animation|SetIsDrawing true)
    (bind _output_get (Variables|Default|SetAnimation%20Index (Math|Integer|SelectInt 1 0 (== (Variables|Default|GetAnimation%20Index) 0))))
    (switch int _output_get
      (:0
        (CallFunction|CloseDrawer))
      (:1
        (CallFunction|OpenDrawer)))))

(fn ConstructionScript
  (|CallParentFunction))