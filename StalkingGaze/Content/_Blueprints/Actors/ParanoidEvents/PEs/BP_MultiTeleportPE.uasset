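; Paranoid event actor that moves a referenced mannequin to the next entry in a list of teleport locations each time InvokeEvent fires.
; It teleports the mannequin using GetLocationAndRotation, keeping its scale, then swaps its skeletal mesh if the parallel Mesh array holds a valid asset.
; The index advances only when the Mesh array has a matching slot, and out-of-range indices print on-screen errors.
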(event EventInvokeEvent
  (bind (_returnvalue _rotation) (Utilities|GetLocationandRotation))
  (bind _index (Variables|Default|GetIndex))
  (bind _mannequinntomove (Variables|Default|GetMannequinnToMove))
  (bind _index_2 (Variables|Default|GetIndex))
  (bind _mesh (Variables|Default|GetMesh))
  (bind _index_3 (Variables|Default|GetIndex))
  (bind _output (Utilities|Array|Get(acopy) _mesh _index_3))
  (if (Utilities|Array|IsValidIndex (Variables|Default|GetTeleportLocations) _index)
    (Transformation|SetActorTransform _mannequinntomove (Math|Transform|MakeTransform _returnvalue _rotation (Transformation|GetActorScale3D _mannequinntomove)) false true)
    (if (Utilities|Array|IsValidIndex (Variables|Default|GetMesh) _index_2)
      (Utilities|IsValid _output
        (:Is%20Valid
          (Components|SkeletalMesh|SetSkeletalMeshAsset (Variables|/Script/Engine.SkeletalMeshActor|GetSkeletalMeshComponent (Variables|Default|GetMannequinnToMove)) _output))
        (:Is%20Not%20Valid
          _))
      (Math|Integer|IncrementInt (Variables|Default|GetIndex))
      (else
        (Development|PrintString (Utilities|String|Append "Index " (Utilities|String|ToString(Integer) _index_2) " invalido en el array de meshes. " " Los 2 arrays tienen que tener el mismo tamaño, si no queres que cambie el mesh dejalo vacio, solo se cambia si hay uno distinto") true true "(R=1.000000,G=0.000000,B=0.178082,A=1.000000)" 5e+01)))
    (else
      (Development|PrintString (Utilities|String|Append "Transform invalid index: " (Utilities|String|ToString(Integer) _index)) true true "(R=1.000000,G=0.000000,B=0.178082,A=1.000000)" 5e+01))))

(fn ConstructionScript)