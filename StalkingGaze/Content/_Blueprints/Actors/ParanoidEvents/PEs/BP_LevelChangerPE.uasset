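; BP_LevelChangerPE is a paranoid event actor that moves the player to another level when invoked.
; InvokeEvent shows a WBP_FadeIn widget, plays its fade and blocks move and look input on the player controller.
; After a short delay it restores input and opens the level referenced by LevelToOpen.
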(event EventInvokeEvent
  (bind _returnvalue (Game|GetPlayerController 0))
  (bind _returnvalue_2 (Game|GetPlayerController 0))
  (bind _returnvalue_3 (UserInterface|CreateWidget "/Game/_Blueprints/Widgets/WBP_FadeIn.WBP_FadeIn_C"))
  (Default|Fadein _returnvalue_3)
  (UserInterface|Viewport|AddtoViewport _returnvalue_3 0)
  (Input|SetIgnoreMoveInput _returnvalue_2 true)
  (Input|SetIgnoreLookInput _returnvalue_2 true)
  (Utilities|FlowControl|Delay 1.3)
  (Input|SetIgnoreMoveInput _returnvalue false)
  (Input|SetIgnoreLookInput _returnvalue false)
  (Game|OpenLevel(byObjectReference) (Variables|Default|GetLevelToOpen)))

(fn ConstructionScript
  (|CallParentFunction))