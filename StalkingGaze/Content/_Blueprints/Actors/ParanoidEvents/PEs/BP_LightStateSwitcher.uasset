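; Paranoid event actor that steps a set of lights through an array of intensity and color states.
; InvokeEvent waits a start delay, then runs a looping timer that lerps every light between the current and next state.
; After each transition and hold delay it advances to the next state, clearing the timer when none remain.
; The construction script can preview the first state in the editor and takes its start delay from it.
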(event EventBeginPlay
  (CallFunction|FChangeState))

(event EventInvokeEvent
  (Utilities|FlowControl|Delay (Variables|Default|GetBeginStateDelay))
  (Utilities|Time|SetTimerbyFunctionName 0 "f_HandleLights" (Variables|Default|GetTickTime) true))

(fn ConstructionScript
  (if (and (Utilities|Array|IsValidIndex (Variables|ParanoidEvent|Lights|GetLightStates)) (Variables|Debugging|GetSetColorInEditor))
    (bind _output_get (Variables|Default|SetCurrentLightState (Utilities|Array|Get(acopy) (Variables|ParanoidEvent|Lights|GetLightStates))))
    (Variables|Default|SetBeginStateDelay (.DelayForNextState (Utilities|Struct|BreakLightStateStruct _output_get)))
    (Utilities|SetLightsLerpAlpha 0.0)))

(fn FHandleLights
  (bind _currentlightstate (Variables|Default|GetCurrentLightState))
  (bind (_transitiontime _delayfornextstate) (Utilities|Struct|BreakLightStateStruct _currentlightstate))
  (bind _output_get (Utilities|TimeElapse))
  (if (< (Variables|Default|GetSwitchingTimer) _transitiontime)
    (Utilities|SetLightsLerpAlpha (Math|Float|SafeDivide _output_get _transitiontime))
    (elif (not (< (- (Variables|Default|GetSwitchingTimer) _transitiontime) _delayfornextstate))
      (Utilities|FlowControl|Sequence
        (:then_0
          (Utilities|SetLightsLerpAlpha 1.0))
        (:then_1
          (if (Utilities|CanChangeState)
            (CallFunction|FChangeState)
            (else
              (Utilities|Time|ClearTimerbyFunctionName 0 "f_HandleLights"))))))))

(fn FChangeState
  (bind _stateindex (Variables|Default|GetStateIndex))
  (if (Utilities|CanChangeState)
    (Variables|Default|SetCurrentLightState (Utilities|Array|Get(acopy) (Variables|ParanoidEvent|Lights|GetLightStates) _stateindex))
    (Variables|Default|SetNextState (Utilities|Array|Get(acopy) (Variables|ParanoidEvent|Lights|GetLightStates) (+ _stateindex 1)))
    (Math|Integer|IncrementInt (Variables|Default|GetStateIndex)
      (:%20%20
        (Variables|Default|SetSwitchingTimer 0.0)
        (return)))))