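; Paranoid event actor that teleports a set of skeletal mesh actors to paired transforms while the player is not looking.
; When invoked, each actor moves only if it is out of view or behind an obstacle and its destination is not in front of the player.
; A sound plays at the first successful move, guarded by a DoOnce.
; Construction draws optional debug arrows from actors to destinations, and BeginPlay draws spheres at the destinations.
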(event EventUpdateDebugSymbols
  (Rendering|Debug|FlushPersistentDebugLines)
  (if (Variables|Default|GetShowDebugElements)
    (for _index (range 0 (- (Utilities|Array|Length (Variables|ParanoidEvent|GetSkeletalMeshes)) 1))
      (Rendering|Debug|DrawDebugArrow (Transformation|GetActorLocation (Utilities|Array|Get(acopy) (Variables|ParanoidEvent|GetSkeletalMeshes) _index)) (.Location (Math|Transform|BreakTransform (Utilities|AddActorOffset (Utilities|Array|Get(acopy) (Variables|ParanoidEvent|GetTeleportLocations) _index)))) 0.0 (select (== (Math|Integer|%(Integer) _index 2) 0) "(R=0.834525,G=1.000000,B=0.000000,A=1.000000)" "(R=0.000000,G=1.000000,B=0.434016,A=1.000000)") 9e+01 3.0))))

(event EventBeginPlay
  (for _array_element (Variables|ParanoidEvent|GetTeleportLocations)
    (Rendering|Debug|DrawDebugSphere (.Location (Math|Transform|BreakTransform (Utilities|AddActorOffset _array_element))) 1e+01 12 "(R=0.806653,G=0.799631,B=1.000000,A=1.000000)" 1e+02)))

(event EventInvokeEvent
  (bind _returnvalue (Game|Player|GetPlayerPawn 0))
  (bind _returnvalue_2 (Game|Player|GetPlayerPawn 0))
  ;[1 1 1 1 35] Invoke Event
  ;;[1 1 1] Checks if the player sees the skms to move
  (for (_array_element _array_index) (Variables|ParanoidEvent|GetSkeletalMeshes)
    (bind _output_get (Variables|Default|SetCurrentActor _array_element))
    (if (or (Default|FIsOutOfView (Variables|Default|GetLineOfSight) 9e+01 (Transformation|GetActorForwardVector _returnvalue_2) (- (Transformation|GetActorLocation _returnvalue_2) (Transformation|GetActorLocation (Variables|Default|GetCurrentActor)))) (Default|FExistObstacleBetween (Variables|Default|GetLineOfSight) (Variables|Default|GetCurrentActor) (Game|Player|GetPlayerPawn 0)))
      (if (not (< (Math|Vector|DotProduct (Transformation|GetActorForwardVector _returnvalue) (- (Transformation|GetActorLocation _returnvalue) (.Location (Math|Transform|BreakTransform (Utilities|AddActorOffset (Utilities|Array|Get(acopy) (Variables|ParanoidEvent|GetTeleportLocations) _array_index) (Transformation|GetActorScale3D (Variables|Default|GetCurrentActor))))))) -1.0))
        ;;[0 1 0.01757] Succeded
        (Transformation|SetActorTransform (Variables|Default|GetCurrentActor) (Utilities|AddActorOffset (Utilities|Array|Get(acopy) (Variables|ParanoidEvent|GetTeleportLocations) _array_index) (Transformation|GetActorScale3D (Variables|Default|GetCurrentActor))) false true)
        (Utilities|FlowControl|DoOnce false
          (:Completed
            (Audio|PlaySoundatLocation (Variables|Default|GetPlayedSound) (Transformation|GetActorLocation (Variables|Default|GetCurrentActor)) "0, 0, 0" 1.0 1.0 0.0 0 0 0 0))))
      (else
        (Development|PrintString (Utilities|String|Append (Utilities|GetDisplayName _output_get) " WAS IN LINE OF SIGHT") true true "(R=1.000000,G=0.025666,B=0.125328,A=1.000000)")))))

(event EventTick
  (params (DeltaSeconds :type Float%20%28single-precision%29))
  (Rendering|Debug|DrawDebugLine "0, 0, 0" "0, 0, 0" "(R=0.000000,G=0.000000,B=0.000000,A=1.000000)" 0.001 0.0))

(fn ConstructionScript
  (|CallParentFunction)
  (Class|ParanoidEvent|UpdateDebugSymbols))