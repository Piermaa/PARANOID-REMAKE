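; A paranoid event actor that plays a set of sounds at locations offset from its own position when invoked.
; InvokeEvent pairs SoundsToPlay and SoundLocations by index, playing each sound with a shared volume multiplier and default attenuation.
; UpdateDebugSymbols redraws temporary debug spheres at those locations and calls InvokeEvent inside the loop, so the full set replays once per location.
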(event EventUpdateDebugSymbols
  (Rendering|Debug|FlushPersistentDebugLines)
  (for _index (range 0 (- (Utilities|Array|Length (Variables|ParanoidEvent|GetSoundLocations)) 1))
    (Rendering|Debug|DrawDebugSphere (+ (Utilities|Array|Get(acopy) (Variables|ParanoidEvent|GetSoundLocations) _index) (Transformation|GetActorLocation)) 5e+02 12 "(R=0.291353,G=0.087070,B=1.000000,A=1.000000)" 1e+01)
    (Class|ParanoidEvent|InvokeEvent)))

(event EventInvokeEvent
  (for _index (range 0 (- (Utilities|Array|Length (Variables|ParanoidEvent|GetSoundLocations)) 1))
    (Audio|PlaySoundatLocation (Utilities|Array|Get(acopy) (Variables|ParanoidEvent|GetSoundsToPlay) _index) (+ (Utilities|Array|Get(acopy) (Variables|ParanoidEvent|GetSoundLocations) _index) (Transformation|GetActorLocation)) "0, 0, 0" (Variables|ParanoidEvent|GetVolume%20Multiplier) 1.0 0.0 "/Game/Audio/Attenuation/SAtt_Default.SAtt_Default" 0 0 0)))

(fn ConstructionScript
  (|CallParentFunction))