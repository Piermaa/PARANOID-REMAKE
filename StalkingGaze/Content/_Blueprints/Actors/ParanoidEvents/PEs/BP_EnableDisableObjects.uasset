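; Paranoid-event actor that enables, disables and destroys lists of level actors when invoked, immediately or after a timer.
; FSetActive toggles visibility and collision, also updating mesh components on StaticMeshActors.
; The event plays a one-shot sound at an offset and up to two loop sounds, sending them an OnStop trigger after a delay.
; The construction script can draw color-coded debug lines to each affected actor.
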(event Custom|DelayedInvoke
  (bind _oneventinvokedloopsfx (Variables|Default|GetOnEventInvokedLoopSFX))
  (bind _oneventinvokedloopsfx2 (Variables|Default|GetOnEventInvokedLoopSFX2))
  (for _array_element (Variables|Default|GetActorsToDisable)
    (CallFunction|FSetActive true _array_element))
  (for _array_element_2 (Variables|Default|GetActorsToEnable)
    (CallFunction|FSetActive false _array_element_2))
  (for _array_element_3 (Variables|Default|GetActorsToDESTROY)
    (Actor|DestroyActor _array_element_3))
  (Audio|PlaySoundatLocation (Variables|Default|GetOnEventInvokedOneShotSFX) (+ (Variables|Default|GetSoundLocation) (Transformation|GetActorLocation)) "0, 0, 0" 1.0 1.0 0.0 "/Game/Audio/Attenuation/SAtt_Default.SAtt_Default" 0 0 0)
  (Utilities|FlowControl|Sequence
    (:then_0
      (Utilities|IsValid _oneventinvokedloopsfx
        (:Is%20Valid
          (bind _returnvalue (Audio|SpawnSoundatLocation _oneventinvokedloopsfx (+ (Variables|Default|GetSoundLocation) (Transformation|GetActorLocation)) "0, 0, 0" 1.0 1.0 0.0 "/Game/Audio/Attenuation/SAtt_Default.SAtt_Default" 0))
          (Variables|Default|SetCachedAudioComp _returnvalue)
          (Utilities|FlowControl|Delay (Variables|Default|GetLoopSoundKillDelay))
          (bind _cachedaudiocomp (Variables|Default|GetCachedAudioComp)
            (:then
              (Class|AudioParameterControllerInterface|SetTriggerParameter _cachedaudiocomp "OnStop"))
            (:else)))))
    (:then_1
      (Utilities|IsValid _oneventinvokedloopsfx2
        (:Is%20Valid
          (bind _returnvalue_2 (Audio|SpawnSoundatLocation _oneventinvokedloopsfx2 (+ (Variables|Default|GetSoundLocation) (Transformation|GetActorLocation)) "0, 0, 0" 1.0 1.0 0.0 "/Game/Audio/Attenuation/SAtt_Default.SAtt_Default" 0))
          (Variables|Default|SetCachedAudioComp2 _returnvalue_2)
          (Utilities|FlowControl|Delay (Variables|Default|GetLoopSoundKillDelay))
          (bind _cachedaudiocomp2 (Variables|Default|GetCachedAudioComp2)
            (:then
              (Class|AudioParameterControllerInterface|SetTriggerParameter _cachedaudiocomp2 "OnStop"))
            (:else)))))))

(event EventUpdateDebugSymbols
  (if (Variables|Default|GetShowDebugElements)
    (Rendering|Debug|FlushPersistentDebugLines)
    (CallFunction|DrawLines (Variables|Default|GetActorsToEnable) "(R=0.000000,G=0.828125,B=0.196199,A=1.000000)")
    (CallFunction|DrawLines (Variables|Default|GetActorsToDisable) "(R=0.828125,G=0.686440,B=0.051518,A=1.000000)")
    (CallFunction|DrawLines (Variables|Default|GetActorsToDESTROY) "(R=0.828125,G=0.000000,B=0.053988,A=1.000000)")
    (else
      (Rendering|Debug|FlushPersistentDebugLines))))

(event EventInvokeEvent
  (if (== (Variables|ParanoidEvent|GetDelayTime) 0.0)
    (CallFunction|DelayedInvoke)
    (else
      (Utilities|Time|SetTimerbyEvent (delegate Custom|DelayedInvoke) (Variables|ParanoidEvent|GetDelayTime)))))

(fn ConstructionScript
  (|CallParentFunction)
  (Class|ParanoidEvent|UpdateDebugSymbols))

(fn DrawLines
  (params (Array :type Array%20of%20Actor%20Object%20References) (LineColor :type Linear%20Color%20Structure))
  (for _array_element Array
    (Utilities|IsValid _array_element
      (:Is%20Valid
        (Rendering|Debug|DrawDebugLine (Transformation|GetActorLocation) (Transformation|GetActorLocation _array_element) LineColor 9e+01 0.0))))
  (return))

(fn FSetActive
  (params (Disabled? :type Boolean) (Actor :type Actor%20Object%20Reference))
  (bind _returnvalue (Actor|GetComponentsByClass Actor "/Script/Engine.StaticMeshComponent"))
  (if (Utilities|IsValid Actor)
    (LocalVariables|SetP_NewActive Disabled?)
    (Rendering|SetActorHiddenInGame Actor (LocalVariables|GetP_NewActive))
    (Collision|SetActorEnableCollision Actor (not (LocalVariables|GetP_NewActive)))
    (bind _asstatic_mesh_actor (Utilities|Casting|CastToStaticMeshActor Actor))
    (Rendering|SetVisibility (Variables|/Script/Engine.StaticMeshActor|GetStaticMeshComponent _asstatic_mesh_actor) (not (LocalVariables|GetP_NewActive)) true)
    (Collision|SetActorEnableCollision _asstatic_mesh_actor (not (LocalVariables|GetP_NewActive)))
    (for _index (range 0 (- (Utilities|Array|Length _returnvalue) 1))
      (Utilities|IsValid (Utilities|Array|Get(acopy) _returnvalue _index)
        (:Is%20Valid
          (Development|SetHiddeninGame (Utilities|Array|Get(acopy) _returnvalue _index) (LocalVariables|GetP_NewActive) true)
          (Collision|SetCollisionEnabled (Utilities|Array|Get(acopy) _returnvalue _index) (select (not (LocalVariables|GetP_NewActive)) "QueryAndPhysics" "NoCollision")))))))