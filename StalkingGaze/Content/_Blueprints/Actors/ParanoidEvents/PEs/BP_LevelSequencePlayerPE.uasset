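; Paranoid event that plays a level sequence when invoked, optionally disabling input on the player's pawn during playback.
; On finish it re-enables input, then triggers chained follow-up events from OnFinishEvents.
; Referenced events are invoked directly, while named and const events go through ParanoidGameInstance, after which the finish delegate is unbound.
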(event Custom|OnFinish
  (bind _returnvalue (Game|GetPlayerController 0))
  (bind _onfinishevents (Variables|Default|GetOnFinishEvents))
  (bind (_paranoideventsnames _constparanoidevents) (Utilities|Struct|BreakParanoidEventsBatch _onfinishevents))
  (Input|EnableInput (Pawn|GetControlledPawn _returnvalue) _returnvalue)
  (Utilities|FlowControl|Sequence
    (:then_0
      (for _array_element (Utilities|Struct|BreakParanoidEventsBatch (Variables|Default|GetOnFinishEvents))
        (Class|ParanoidEvent|TryInvokeEvent _array_element)))
    (:then_1
      (bind _asparanoid_game_instance (Utilities|Casting|CastToParanoidGameInstance (Game|GetGameInstance)))
      (Utilities|FlowControl|Sequence
        (:then_0
          (for _array_element_2 _paranoideventsnames
            (Class|ParanoidGameInstance|CallEvents _asparanoid_game_instance _array_element_2)))
        (:then_1
          (for _array_element_3 _constparanoidevents
            (Class|ParanoidGameInstance|CallConstEvents _asparanoid_game_instance _array_element_3))
          (EventDispatchers|UnbindallEventsfromOnFinished (Variables|ParanoidEvent|GetLevelSequencePlayer)))))))

(event EventInvokeEvent
  (bind _returnvalue (Game|GetPlayerController 0))
  (bind _outactor (Sequencer|Player|CreateLevelSequencePlayer (Variables|ParanoidEvent|GetLevel%20Sequence)))
  (Variables|ParanoidEvent|SetLevelSequencePlayer (Variables|/Script/LevelSequence.LevelSequenceActor|GetSequencePlayer _outactor))
  (Sequencer|Player|Play (Variables|/Script/LevelSequence.LevelSequenceActor|GetSequencePlayer _outactor) :!class /Script/MovieScene.MovieSceneSequencePlayer)
  (if (Variables|ParanoidEvent|GetBlocks%20input)
    (Input|DisableInput (Pawn|GetControlledPawn _returnvalue) _returnvalue))
  (EventDispatchers|BindEventtoOnFinished (Variables|/Script/LevelSequence.LevelSequenceActor|GetSequencePlayer _outactor) (EventDispatchers|CreateEvent :!event Custom|OnFinish)))

(fn ConstructionScript
  (|CallParentFunction))