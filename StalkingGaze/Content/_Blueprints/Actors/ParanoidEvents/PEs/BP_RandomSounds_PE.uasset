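; BP_RandomSounds_PE is a paranoid event that plays random sounds at random locations around the player.
; InvokeEvent toggles it, either clearing the running timer or queuing a sound after a random delay, with each PlaySound queuing the next.
; Helper macros pick the sound from an array and offset the location from the player pawn by a scaled random vector, confined to the positive X/Y quadrant at pawn height.
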(event Custom|QueueNewSound
  (bind _randomtimebetweensounds (Variables|ParanoidEvents|GetRandomTimeBetweenSounds))
  (bind (_x _y) (Math|Vector2D|BreakVector2D _randomtimebetweensounds))
  (bind _returnvalue (Utilities|Time|SetTimerbyEvent (EventDispatchers|CreateEvent :!event Custom|PlaySound) (Math|Random|RandomFloatinRange _x _y)))
  (Variables|Default|SetTimer _returnvalue))

(event Custom|PlaySound
  (Audio|PlaySoundatLocation (Utilities|MGetRandomSound) (Utilities|MGetRandomLocation) "0, 0, 0" 1.0 1.0 0.0 "/Game/Audio/Attenuation/SAtt_Default.SAtt_Default" 0 0 0)
  (CallFunction|QueueNewSound))

(event EventInvokeEvent
  (if (Utilities|Time|IsValidTimerHandle (Variables|Default|GetTimer))
    (Utilities|Time|ClearandInvalidateTimerbyHandle (Variables|Default|GetTimer)) ; stops
    (else
      (CallFunction|QueueNewSound) ; start
    )))

(fn ConstructionScript)