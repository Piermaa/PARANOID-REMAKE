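; BP_ReadableDocument is an interactable world document that the player can open and read on screen.
; A data table row supplies its content; the construction script applies that row's image to the mesh through a dynamic material's PosterTexture parameter.
; Interact runs the parent logic, then shows the row in a scaled WBP_Paper widget with UI-only input and a visible cursor.
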(event EventInteract
  (bind _returnvalue (Game|GetPlayerController 0))
  (bind _document (Variables|ParanoidEvents|GetDocument))
  (bind (_datatable _rowname) (Utilities|Struct|BreakDataTableRowHandle _document))
  (|CallParentFunction)
  (bind _returnvalue_2 (Utilities|GetDataTableRow _datatable _rowname)
    (:then
      (bind _returnvalue_3 (UserInterface|CreateWidget "/Game/_Blueprints/Widgets/WBP_Paper.WBP_Paper_C"))
      (Default|UpdateDisplay _returnvalue_3 _returnvalue_2 (Variables|ParanoidEvents|GetDocumentSizeScale))
      (UserInterface|Viewport|AddtoViewport _returnvalue_3 0)
      (Input|SetInputModeUIOnly _returnvalue _returnvalue_3 "DoNotLock" true)
      (Variables|/Script/Engine.PlayerController|SetbShowMouseCursor _returnvalue true))))

(fn ConstructionScript
  (bind _document (Variables|ParanoidEvents|GetDocument))
  (bind _static_mesh (Variables|Default|GetStatic%20Mesh))
  (bind (_datatable _rowname) (Utilities|Struct|BreakDataTableRowHandle _document))
  (|CallParentFunction)
  (Utilities|FlowControl|Sequence
    (:then_0
      (LocalVariables|GetDynamicPosterMaterial
        (:then)
        (:else
          (bind _returnvalue (Rendering|Material|CreateDynamicMaterialInstance _static_mesh 0 (Rendering|Material|GetMaterial _static_mesh 0) "None" :!class /Script/Engine.PrimitiveComponent))
          (LocalVariables|SetDynamicPosterMaterial _returnvalue)
          (Rendering|Material|SetMaterial (Variables|Default|GetStatic%20Mesh) 0 _returnvalue))))
    (:then_1
      (bind _returnvalue_2 (Utilities|GetDataTableRow _datatable _rowname)
        (:then
          (Rendering|Material|SetTextureParameterValue (LocalVariables|GetDynamicPosterMaterial) "PosterTexture" (.Image (Utilities|Struct|BreakF_DocumentsRow _returnvalue_2))))))))