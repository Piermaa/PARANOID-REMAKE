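; Animated interactable Paranoid Event invoker that plays an animation and tries to dispatch paranoid events when interacted with.
; PlayBlueprintAnimation is an empty event here, while start and finish events toggle IsPlayingAnimation.
; On each animation start, a FlipFlop alternates between the first and repeat interaction sounds at the actor's location.
; Animation completion forwards its direction through CallOnAnimationFinish.
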(event Custom|AnimationFinished
  (params (Forward? :type Boolean))
  (Default|CallOnAnimationFinish Forward?)
  (Variables|Default|SetbIsPlayingAnimation false))

(event Custom|AnimationStarted
  (Variables|Default|SetbIsPlayingAnimation true)
  (Utilities|FlowControl|FlipFlop
    (:A
      (Audio|PlaySoundatLocation (Variables|Default|GetOnInteractSFX) (Transformation|GetActorLocation) "0, 0, 0" 1.0 1.0 0.0 "/Game/Audio/Attenuation/SAtt_Default.SAtt_Default" 0 0 0))
    (:B
      (Audio|PlaySoundatLocation (Variables|Default|GetOnInteractAgainSFX) (Transformation|GetActorLocation) "0, 0, 0" 1.0 1.0 0.0 "/Game/Audio/Attenuation/SAtt_Default.SAtt_Default" 0 0 0))))

(event EventInteract
  (CallFunction|PlayBlueprintAnimation)
  (Class|ParanoidEventDispatcher|TryDispatchParanoidEvents))

(event EventPlayBlueprintAnimation
  (params (AnimationIndex :type Integer)))

(fn ConstructionScript
  (|CallParentFunction))