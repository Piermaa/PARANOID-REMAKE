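; Pickupable item actor in the paranoid-event (PE) invoker family, exposing its mesh to be picked up.
; On interaction it runs the parent logic, then hides its main mesh and children in game while setting that mesh visible in ray tracing.
; A second mesh is switched to scene-capture-only visibility.
; Pickup returns the main mesh asset, its materials and a pickup transform to the caller.
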(event EventInteract
  (|CallParentFunction)
  (Development|SetHiddeninGame (Variables|Default|GetStatic%20Mesh) true true)
  (Class|PrimitiveComponent|SetVisibleinRayTracing (Variables|Default|GetStatic%20Mesh) true)
  (Class|PrimitiveComponent|SetVisibleinSceneCaptureOnly (Variables|Default|GetStatic%20Mesh1) true))

(fn ConstructionScript
  (|CallParentFunction))

(fn Pickup
  (bind _static_mesh (Variables|Default|GetStatic%20Mesh))
  (return (Rendering|Material|GetMaterials _static_mesh) (Variables|Default|GetPickupLocation) (Variables|/Script/Engine.StaticMeshComponent|GetStaticMesh _static_mesh)))