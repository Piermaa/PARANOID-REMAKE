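; First-person player character Blueprint handling camera zoom, screen flash, footstep audio and look sensitivity.
; Timelines drive FOV zoom, reversed on release or controller loss, and a flash scalar on a lazily created, cached post-process dynamic material.
; Footstep delegate events trace downward to pick walk or run sounds by physical surface.
; BeginPlay shows a fade widget, caches the HUD, clears game-instance keys and syncs camera sensitivity.
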(event Custom|Play%20Footsteps%20Sound
  (bind _returnvalue (Transformation|GetActorLocation))
  ;[0 0.2372 1] FOOTSTEPS
  (if (Variables|Default|GetFootstepsEnabled)
    (bind (_outhit _returnvalue_2) (Collision|LineTraceByChannel _returnvalue (+ _returnvalue "0.000000,0.000000,-300.000000") "TraceTypeQuery1" false 0 "ForDuration" true "(R=1.000000,G=0.000000,B=0.000000,A=1.000000)" "(R=0.000000,G=1.000000,B=0.000000,A=1.000000)" 2.0))
    (if _returnvalue_2
      (if (Class|RealisticRunningComponent|ReachedRunningSpeed (Variables|Default|GetRealisticRunningComponent))
        (switch Utilities|FlowControl|Switch|SwitchonEPhysicalSurface (Variables|/Script/PhysicsCore.PhysicalMaterial|GetSurfaceType (.PhysMat (Collision|BreakHitResult _outhit)))
          (:SurfaceType1
            (Audio|PlaySound2D "/Game/Audio/SoundPresets/Footsteps/MSP_SFX_Footsteps_Wood_Run.MSP_SFX_Footsteps_Wood_Run" 1.0 1.0 0.0 0 0))
          (:SurfaceType2
            (Audio|PlaySound2D "/Game/Audio/SoundPresets/Footsteps/MSP_SFX_Footsteps_Concrete_Run.MSP_SFX_Footsteps_Concrete_Run" 1.0 1.0 0.0 0 0))
          (:SurfaceType3
            (Audio|PlaySound2D "/Game/Audio/SoundPresets/Footsteps/MSP_SFX_Footsteps_Grass_Run.MSP_SFX_Footsteps_Grass_Run" 1.0 1.0 0.0 0 0)))
        (else
          (switch Utilities|FlowControl|Switch|SwitchonEPhysicalSurface (Variables|/Script/PhysicsCore.PhysicalMaterial|GetSurfaceType (.PhysMat (Collision|BreakHitResult _outhit)))
            (:SurfaceType1
              (Audio|PlaySound2D "/Game/Audio/SoundPresets/Footsteps/MSP_SFX_Footsteps_Wood.MSP_SFX_Footsteps_Wood" 1.0 1.0 0.0 0 0))
            (:SurfaceType2
              (Audio|PlaySound2D "/Game/Audio/SoundPresets/Footsteps/MSP_SFX_Footsteps_Concrete.MSP_SFX_Footsteps_Concrete" 1.0 1.0 0.0 0 0))
            (:SurfaceType3
              (Audio|PlaySound2D "/Game/Audio/SoundPresets/Footsteps/MSP_SFX_Footsteps_Grass.MSP_SFX_Footsteps_Grass" 1.0 1.0 0.0 0 0))))))))

(event Custom|ClearZoom
  (bind _newtrack_0 (Timeline|Timeline Reverse)
    (:Update
      (Camera|SetFieldOfView (Variables|Default|GetCameraComp) (Math|Float|Lerp 9e+01 4e+01 _newtrack_0)))))

(event Custom|SetSensibility
  (params (New%20Sensibility :type Float%20%28double-precision%29))
  ;[0 0.2372 1] FOOTSTEPS
  (Variables|Default|SetCameraSensibility New%20Sensibility))

(event Input|EnhancedActionEvents|EnhancedInputActionIA_Zoom
  (params (ActionValue :type Boolean) (ElapsedSeconds :type Float%20%28double-precision%29) (TriggeredSeconds :type Float%20%28double-precision%29) (InputAction :type Input%20Action%20Object%20Reference :default "/Game/Input/Actions/IA_Zoom.IA_Zoom"))
  (:Started
    (bind _newtrack_0 (Timeline|Timeline Play)
      (:Update
        (Camera|SetFieldOfView (Variables|Default|GetCameraComp) (Math|Float|Lerp 9e+01 4e+01 _newtrack_0)))))
  (:Completed
    (Timeline|Timeline Reverse)))

(event EventBeginPlay
  ;[0 0.2372 1] FOOTSTEPS
  (|CallParentFunction)
  (Utilities|FlowControl|Sequence
    (:then_0
      (EventDispatchers|BindEventtoOnFootstepsDelegate (Variables|Default|GetFootsteps) (EventDispatchers|CreateEvent :!event Custom|Play%20Footsteps%20Sound))
      (bind _returnvalue (UserInterface|CreateWidget "/Game/_Blueprints/Widgets/WBP_FadeIn.WBP_FadeIn_C" (.AsPlayer%20Controller (Utilities|Casting|CastToPlayerController (Pawn|GetController)))))
      (Default|FadeOut _returnvalue)
      (UserInterface|Viewport|AddtoViewport _returnvalue 0))
    (:then_1
      (bind _aspc_first_person_controller (Utilities|Casting|CastToPC_FirstPersonController (Pawn|GetController)))
      (Variables|Default|SetHUD%20Widget (Variables|/Game/_Blueprints/Controller/PC_FirstPersonController.PC_FirstPersonController_C|GetHUD%20Widget _aspc_first_person_controller)))
    (:then_2
      (bind _asbp_paranoid_game_instance (Utilities|Casting|CastToBP_ParanoidGameInstance (Game|GetGameInstance)))
      (bind _output_get (Variables|Default|SetAs%20BP%20Paranoid%20Game%20Instance _asbp_paranoid_game_instance))
      (EventDispatchers|BindEventtoOnSensibilityChange _output_get (EventDispatchers|CreateEvent :!event Custom|SetSensibility))
      (Class|ParanoidGameInstance|ClearKeys _asbp_paranoid_game_instance)
      (if (!= (.CameraSensibility (Utilities|Struct|BreakF_GameConfig (Variables|/Game/_Blueprints/BP_ParanoidGameInstance.BP_ParanoidGameInstance_C|GetGameConfig _asbp_paranoid_game_instance))) 0.0)
        (CallFunction|SetSensibility (.CameraSensibility (Utilities|Struct|BreakF_GameConfig (Variables|/Game/_Blueprints/BP_ParanoidGameInstance.BP_ParanoidGameInstance_C|GetGameConfig _asbp_paranoid_game_instance))))))))

(event EventFnDispatchFlashEffect
  ;[0.6727 1 0.1058] BPI
  (bind _newtrack_0 (Timeline|Flash PlayFromStart)
    (:Update
      (bind _flashmaterial (CallFunction|FGetPostProcessMaterial))
      (Rendering|Material|SetScalarParameterValue _flashmaterial "FlashIntensity" _newtrack_0 :!class /Script/Engine.MaterialInstanceDynamic))))

(event EventControllerChanged
  (params (OldController :type Controller%20Object%20Reference) (NewController :type Controller%20Object%20Reference))
  ;[0 0.2372 1] FOOTSTEPS
  (Utilities|IsValid NewController
    (:Is%20Not%20Valid
      (CallFunction|ClearZoom))))

(event Input|KeyboardEvents|DebugKey0
  (params (Key :type Key%20Structure :default "None") (ActionValue :type Input%20Action%20Value%20Structure))
  (:Pressed
    (bind _outactors (Actor|GetAllActorsOfClass "/Script/Engine.PlayerStart"))
    (Transformation|SetActorLocation (Transformation|GetActorLocation (Utilities|Array|Get(acopy) _outactors)) false true)))

(event Input|KeyboardEvents|DebugKeyT
  (params (Key :type Key%20Structure :default "None") (ActionValue :type Input%20Action%20Value%20Structure))
  ;[0 0.2372 1] FOOTSTEPS
  (:Pressed
    (bind _outactors (Actor|GetAllActorsOfClass "/Game/_Blueprints/Wire/BP_HangingWire.BP_HangingWire_C"))
    (CallFunction|FTEST _outactors)))

(fn ConstructionScript)

(fn FGetPC
  (bind _pc (Variables|Default|GetPC)
    (:then
      (return _pc))
    (:else
      (bind _aspc_first_person_controller (Utilities|Casting|CastToPC_FirstPersonController (Pawn|GetController)))
      (return _aspc_first_person_controller))))

(fn FTEST
  (params (Array :type Array%20of%20BP%20Hanging%20Wire%20Object%20References))
  (for _array_element Array
    (if (Variables|/Game/_Blueprints/Wire/BP_HangingWire.BP_HangingWire_C|GetSimulates _array_element)
      (Math|Integer|IncrementInt (LocalVariables|GetAmount))))
  (return))

(fn FGetPostProcessMaterial
  (bind _cameracomp (Variables|Default|GetCameraComp))
  (bind _flashmaterial (Variables|Default|GetFlashmaterial)
    (:then
      (return _flashmaterial))
    (:else
      (if (Utilities|Array|IsValidIndex (Utilities|Struct|BreakWeightedBlendables (Utilities|Struct|BreakPostProcessSettings (Variables|/Script/Engine.CameraComponent|GetPostProcessSettings _cameracomp))))
        (bind _asmaterial_interface (Utilities|Casting|CastToMaterialInterface (Utilities|Struct|BreakWeightedBlendable (Utilities|Array|Get(acopy) (Utilities|Struct|BreakWeightedBlendables (Utilities|Struct|BreakPostProcessSettings (Variables|/Script/Engine.CameraComponent|GetPostProcessSettings _cameracomp)))))))
        (bind _returnvalue (Rendering|Material|CreateDynamicMaterialInstance _asmaterial_interface "None" "None" :!class /Script/Engine.KismetMaterialLibrary))
        (bind _structout (Utilities|Struct|SetmembersinWeightedBlendable (Utilities|Array|Get(acopy) (Utilities|Struct|BreakWeightedBlendables (Utilities|Struct|BreakPostProcessSettings (Variables|/Script/Engine.CameraComponent|GetPostProcessSettings _cameracomp)))) _returnvalue))
        (Utilities|Array|SetArrayElem (Utilities|Struct|BreakWeightedBlendables (Utilities|Struct|BreakPostProcessSettings (Variables|/Script/Engine.CameraComponent|GetPostProcessSettings _cameracomp))) 0 _structout)
        (bind _structout_2 (Utilities|Struct|SetmembersinWeightedBlendables (Utilities|Struct|BreakPostProcessSettings (Variables|/Script/Engine.CameraComponent|GetPostProcessSettings _cameracomp)) (Utilities|Struct|BreakWeightedBlendables (Utilities|Struct|BreakPostProcessSettings (Variables|/Script/Engine.CameraComponent|GetPostProcessSettings _cameracomp)))))
        (bind _structout_3 (Utilities|Struct|SetmembersinPostProcessSettings (Variables|/Script/Engine.CameraComponent|GetPostProcessSettings _cameracomp) _structout_2))
        (Variables|/Script/Engine.CameraComponent|SetPostProcessSettings _cameracomp _structout_3)
        (bind _output_get (Variables|Default|SetFlashmaterial _returnvalue))
        (return _output_get)))))