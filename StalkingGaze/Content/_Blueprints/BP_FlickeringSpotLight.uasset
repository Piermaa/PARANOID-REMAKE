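; Spotlight Blueprint whose brightness flickers during play, with configurable color, radius and cone.
; On BeginPlay a timeline drives a lerp between low and high flicker intensities, scaled by brightness and an intensity multiplier.
; The construction script applies color and attenuation radius, but feeds InnerConeAngle into the outer cone setter.
; The setter using OuterConeAngle is disconnected, so that value has no effect.
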(event EventBeginPlay
  (bind _newtrack_0 (Timeline|Timeline_0 Play)
    (:Update
      (Rendering|Components|Light|SetIntensity (Variables|Default|GetSpotLight) (* (* (Variables|Default|GetLightBrightness) (Variables|Default|GetLightScaleIntensity)) (Math|Float|Lerp (Variables|Default|GetFlickerIntensityLow) (Variables|Default|GetFlickerIntensityHigh) _newtrack_0))))))

(fn ConstructionScript
  (bind _spotlight (Variables|Default|GetSpotLight))
  (Rendering|Components|Light|SetLightColor _spotlight (Variables|Lights|GetColor) true)
  (Rendering|Lighting|SetAttenuationRadius _spotlight (Variables|Lights|GetRadius))
  (Rendering|Lighting|SetOuterConeAngle _spotlight (Variables|Lights|GetInner%20Cone%20Angle)))