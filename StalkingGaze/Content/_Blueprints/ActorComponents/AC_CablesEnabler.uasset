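; Actor component that toggles physics on wires as they enter and leave its owner's sphere component, presumably to limit simulation to nearby cables.
; Begin overlap enables physics on actors implementing BPI_Wire if it is off, and end overlap disables it.
; It also caches the owner's LineOfSight component and starts a looping timer, but the field-of-view check is disconnected, leaving CheckWireInLOS empty and only overlaps driving physics.
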(event Custom|OnBeginOverlap
  (params (OverlappedComponent :type Primitive%20Component%20Object%20Reference) (OtherActor :type Actor%20Object%20Reference) (OtherComp :type Primitive%20Component%20Object%20Reference) (OtherBodyIndex :type Integer) (bFromSweep :type Boolean) (SweepResult :type Hit%20Result%20Structure%20%28by%20ref%29))
  (if (Utilities|DoesObjectImplementInterface OtherActor "/Game/_Blueprints/Wire/BPI_Wire.BPI_Wire_C")
    (bind _value (Class|BPIWire|FnGetPhysicsEnabled(Message) OtherActor))
    (if (not _value)
      (Class|BPIWire|FnSetPhysics(Message) OtherActor true))))

(event Custom|OnComponentEndOverlap_Event
  (params (OverlappedComponent :type Primitive%20Component%20Object%20Reference) (OtherActor :type Actor%20Object%20Reference) (OtherComp :type Primitive%20Component%20Object%20Reference) (OtherBodyIndex :type Integer))
  (if (Utilities|DoesObjectImplementInterface OtherActor "/Game/_Blueprints/Wire/BPI_Wire.BPI_Wire_C")
    (Class|BPIWire|FnSetPhysics(Message) OtherActor false)))

(event Custom|CheckWireInLOS)

(event EventBeginPlay
  (bind _returnvalue (Components|GetOwner))
  (bind _returnvalue_2 (Actor|GetComponentbyClass _returnvalue "/Script/Engine.SphereComponent"))
  (Utilities|FlowControl|Sequence
    (:then_0
      (Variables|Default|SetSphere _returnvalue_2)
      (Collision|BindEventtoOnComponentBeginOverlap _returnvalue_2 (EventDispatchers|CreateEvent :!event Custom|OnBeginOverlap))
      (Collision|AssignOnComponentEndOverlap _returnvalue_2 (EventDispatchers|CreateEvent :!event Custom|OnComponentEndOverlap_Event)))
    (:then_1
      (Variables|Default|SetLOS (Actor|GetComponentbyClass (Components|GetOwner) "/Game/_Blueprints/ActorComponents/LineOfSight.LineOfSight_C"))
      (Utilities|Time|SetTimerbyEvent (EventDispatchers|CreateEvent :!event Custom|CheckWireInLOS) 0.2 true))))