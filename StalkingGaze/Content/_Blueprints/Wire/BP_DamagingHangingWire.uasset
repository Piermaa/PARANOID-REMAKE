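; Hanging wire actor that attaches configurable decoration actors along a simulated Cable component.
; The construction script spawns each DecorationPieces entry as a child actor, clamps its section to the segment count, stores the component reference and applies location and yaw.
; Tick teleports each piece to its cable particle location so it follows the simulation, without updating rotation.
; No damage logic appears in these graphs despite the asset's name.
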(event EventBeginPlay
  (|CallParentFunction) ; This node is disabled and will not be called.\nDrag off pins to build functionality.
)

(event Collision|EventActorBeginOverlap
  (params (OtherActor :type Actor%20Object%20Reference)))

(event EventTick
  (params (DeltaSeconds :type Float%20%28single-precision%29))
  (for _array_element (Variables|Default|GetDecorationPieces)
    (Transformation|SetWorldLocation (.__InternalRef (Utilities|Struct|Breakf_DamagingWireStruct _array_element)) (Utilities|Array|Get(acopy) (Class|CableComponent|GetCableParticleLocations (Variables|Default|GetCable)) (.Section (Utilities|Struct|Breakf_DamagingWireStruct _array_element))) false true)))

(fn ConstructionScript
  (bind _cable (Variables|Default|GetCable))
  (bind _locations (Class|CableComponent|GetCableParticleLocations _cable))
  (|CallParentFunction)
  (for (_array_element _array_index) (Variables|Default|GetDecorationPieces)
    (bind _returnvalue (AddComponent|AddChildActorComponent false))
    (ChildActorComponent|SetChildActorClass _returnvalue (.Class (Utilities|Struct|Breakf_DamagingWireStruct _array_element)))
    (bind _structout (Utilities|Struct|Setmembersinf_DamagingWireStruct _array_element (Math|Integer|Clamp(Integer) (.Section (Utilities|Struct|Breakf_DamagingWireStruct _array_element)) 0 (- (Variables|/Script/CableComponent.CableComponent|GetNumSegments (Variables|Default|GetCable)) 1)) _returnvalue))
    (Utilities|Array|SetArrayElem (Variables|Default|GetDecorationPieces) _array_index _structout)
    (if (Utilities|Array|IsValidIndex _locations (.Section (Utilities|Struct|Breakf_DamagingWireStruct _array_element)))
      (Transformation|SetWorldLocationAndRotation _returnvalue (Utilities|Array|Get(acopy) _locations (.Section (Utilities|Struct|Breakf_DamagingWireStruct _array_element))) (Math|Rotator|MakeRotator 0.0 0.0 (.Yaw (Utilities|Struct|Breakf_DamagingWireStruct _array_element))) false true))))