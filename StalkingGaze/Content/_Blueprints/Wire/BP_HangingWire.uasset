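; Hanging wire actor whose sphere can swing under physics and notifies when it hits the player.
; Enabling physics applies a random horizontal impulse after a random delay; disabling it uses a timeline to sweep the sphere back to its starting position.
; Player hits pass through a gate that closes immediately and reopens via a retriggerable delay, so continuous contact fires the hit notification only once.
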(event OnComponentHit(Sphere)
  (params (HitComponent :type Primitive%20Component%20Object%20Reference) (OtherActor :type Actor%20Object%20Reference) (OtherComp :type Primitive%20Component%20Object%20Reference) (NormalImpulse :type Vector :default "0, 0, 0") (Hit :type Hit%20Result%20Structure%20%28by%20ref%29))
  (if (== OtherActor (Game|Player|GetPlayerPawn 0))
    (Utilities|FlowControl|Sequence
      (:then_0
        (Utilities|FlowControl|RetriggerableDelay 1.0)
        (CallFunction|OpenDamageGate))
      (:then_1
        (Utilities|FlowControl|Gate false
          (:Exit
            (CallFunction|CloseDamageGate)
            (Default|CallOnPlayerHit)))))))

(event Custom|OpenDamageGate
  (Utilities|FlowControl|Gate false) ; enters at Open
)

(event Custom|CloseDamageGate
  (Utilities|FlowControl|Gate false) ; enters at Close
)

(event Custom|StopTimeline
  (bind _newtrack_0 (Timeline|Timeline Stop)
    (:Update
      (Transformation|SetWorldLocation (Variables|Default|GetSphere) (Math|Vector|Lerp(Vector) (Variables|Default|GetPhxPos) (Variables|Default|GetStartingPos) _newtrack_0) true false))))

(event EventFnSetPhysics
  (params (NowEnabled :type Boolean))
  (bind _returnvalue (Math|Random|RandomBool))
  (bind _returnvalue_2 (Math|Random|RandomFloatinRange 5e+01 1e+02))
  (bind _returnvalue_3 (Math|Random|RandomFloatinRange -1e+02 -5e+01))
  (bind _returnvalue_4 (Math|Float|SelectFloat _returnvalue_3 _returnvalue_2 _returnvalue))
  (Variables|Default|SetSimulates NowEnabled)
  (Physics|SetSimulatePhysics (Variables|Default|GetSphere) NowEnabled)
  (if NowEnabled
    (Utilities|FlowControl|Delay (Math|Random|RandomFloat))
    (Physics|AddImpulse (Variables|Default|GetSphere) (Math|Vector|MakeVector _returnvalue_4 _returnvalue_4 0.0) "None" true)
    (CallFunction|StopTimeline)
    (else
      (Variables|Default|SetPhxPos (Transformation|GetWorldLocation (Variables|Default|GetSphere)))
      (bind _newtrack_0 (Timeline|Timeline PlayFromStart)
        (:Update
          (Transformation|SetWorldLocation (Variables|Default|GetSphere) (Math|Vector|Lerp(Vector) (Variables|Default|GetPhxPos) (Variables|Default|GetStartingPos) _newtrack_0) true false))))))

(event EventBeginPlay
  (Variables|Default|SetStartingPos (Transformation|GetWorldLocation (Variables|Default|GetSphere))))

(fn ConstructionScript)

(fn FnGetPhysicsEnabled
  (return (Variables|Default|GetSimulates)))