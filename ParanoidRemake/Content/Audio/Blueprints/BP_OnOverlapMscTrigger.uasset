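; BP_OnOverlapMscTrigger is a box trigger that plays a music track while the player character is inside it.
; Begin overlap sends a play message with the track and fade times to the Game Instance, and end overlap sends a stop message with the fade-out time.
; Exiting sets a played flag, which blocks further play and stop messages when DontPlayAgainAfterStopping is enabled.
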(event OnComponentBeginOverlap(Box)
  (params (OverlappedComponent :type Primitive%20Component%20Object%20Reference) (OtherActor :type Actor%20Object%20Reference) (OtherComp :type Primitive%20Component%20Object%20Reference) (OtherBodyIndex :type Integer) (bFromSweep :type Boolean) (SweepResult :type Hit%20Result%20Structure%20%28by%20ref%29))
  (if (Variables|Default|GetbDontPlayAgainAfterStopping)
    (if (not (Variables|Default|GetbHasAlreadyPlayedOnce))
      (Utilities|Casting|CastToPlayerCharacter OtherActor :!label _label)
      (Class|BPIMusicPlayer|PlayMusic(Message) (Game|GetGameInstance) (Variables|Default|GetMusic) (Variables|Default|GetFInTime) (Variables|Default|GetFOutTime)))
    (else
      (goto _label))))

(event OnComponentEndOverlap(Box)
  (params (OverlappedComponent :type Primitive%20Component%20Object%20Reference) (OtherActor :type Actor%20Object%20Reference) (OtherComp :type Primitive%20Component%20Object%20Reference) (OtherBodyIndex :type Integer))
  (if (Variables|Default|GetbDontPlayAgainAfterStopping)
    (if (not (Variables|Default|GetbHasAlreadyPlayedOnce))
      (Utilities|Casting|CastToPlayerCharacter OtherActor :!label _label)
      (Class|BPIMusicPlayer|StopMusic(Message) (Game|GetGameInstance) (Variables|Default|GetFOutTime))
      (Variables|Default|SetbHasAlreadyPlayedOnce true))
    (else
      (goto _label))))

(fn ConstructionScript)