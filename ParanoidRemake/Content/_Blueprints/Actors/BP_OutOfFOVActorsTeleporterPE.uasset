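; Actor that teleports a set of skeletal mesh actors to preset transforms while they are out of the player's view.
; InvokeEvent loops over SkeletalMeshes and moves only those not rendered in roughly the last frame, skipping visible ones.
; Each takes the TeleportLocations entry at the same index, with location offset from this actor's position and rotation and scale applied as stored.
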(event EventBeginPlay)

(event EventInvokeEvent
  (for (_array_element _array_index) (Variables|ParanoidEvent|GetSkeletalMeshes)
    (Variables|Default|SetCurrentActor _array_element)
    (if (not (Class|Actor|WasRecentlyRendered (Variables|Default|GetCurrentActor) 0.016))
      (Transformation|SetActorTransform (Variables|Default|GetCurrentActor) (Math|Transform|MakeTransform (+ (.Location (Math|Transform|BreakTransform (Utilities|Array|Get(acopy) (Variables|ParanoidEvent|GetTeleportLocations) _array_index))) (Transformation|GetActorLocation)) (.Rotation (Math|Transform|BreakTransform (Utilities|Array|Get(acopy) (Variables|ParanoidEvent|GetTeleportLocations) _array_index))) (.Scale (Math|Transform|BreakTransform (Utilities|Array|Get(acopy) (Variables|ParanoidEvent|GetTeleportLocations) _array_index)))) false true))))

(fn ConstructionScript)