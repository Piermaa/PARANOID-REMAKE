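; BP_TriggerPEInvoker is a trigger volume that dispatches paranoid events when the player enters it.
; On overlap, if PlayerTrigger is set, it checks for player pawn 0, asks the Game Instance about required keys, then dispatches after TriggerDelay.
; BeginPlay draws a temporary randomly colored debug box around the collision bounds.
; The construction script toggles the debug cube's visibility.
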(event OnComponentBeginOverlap(BoxCollision)
  (params (OverlappedComponent :type Primitive%20Component%20Object%20Reference) (OtherActor :type Actor%20Object%20Reference) (OtherComp :type Primitive%20Component%20Object%20Reference) (OtherBodyIndex :type Integer) (bFromSweep :type Boolean) (SweepResult :type Hit%20Result%20Structure%20%28by%20ref%29))
  (if (Variables|Default|GetPlayerTrigger)
    (if (== OtherActor (Game|Player|GetPlayerPawn 0))
      (bind _keysrequiredtouse (Class|KeyLockedActorInterface|KeysRequiredtoUse))
      (bind _returnvalue (Class|KeyHolderActor|ActorHasKeys(Message) (Game|GetGameInstance) _keysrequiredtouse))
      (if _returnvalue
        (Utilities|FlowControl|Delay (Variables|ParanoidEvent|GetTriggerDelay))
        (Class|ParanoidEventDispatcher|DispatchParanoidEvents)))))

(event EventBeginPlay
  (bind _boxcollision (Variables|Default|GetBoxCollision))
  (Rendering|Debug|DrawDebugBox (Transformation|GetWorldLocation _boxcollision) (Components|Box|GetScaledBoxExtent _boxcollision) (Utilities|Select :Index (Math|Random|RandomInteger 4) :Option%200 "(R=0.000000,G=1.000000,B=0.128237,A=1.000000)" :Option%201 "(R=0.029578,G=0.416667,B=0.031531,A=1.000000)" :Option%202 "(R=0.043650,G=1.000000,B=0.474044,A=1.000000)" :Option%203 "(R=0.000000,G=0.634885,B=0.901042,A=1.000000)" :Option%204 "(R=0.524994,G=1.000000,B=0.010197,A=1.000000)") "0, 0, 0" 1e+02 1.0))

(fn ConstructionScript
  (Rendering|SetVisibility (Variables|Default|GetCube) (Variables|Default|GetDebugCubeVisibility) false))