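; Paranoid event actor that, when invoked, teleports a list of actors to preset transforms while the player is not looking.
; Each entry in SkeletalMeshes pairs by index with a TeleportLocations transform, passed through AddActorOffset, and moves only if it was not just rendered.
; In construction, an optional debug view draws alternately colored arrows from each actor to its destination, or flushes debug lines when disabled.
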(event EventBeginPlay)

(event EventUpdateDebugSymbols
  (if (Variables|Default|GetShowDebugElements)
    (for _index (range 0 (- (Utilities|Array|Length (Variables|ParanoidEvent|GetSkeletalMeshes)) 1))
      (Rendering|Debug|DrawDebugArrow (Transformation|GetActorLocation (Utilities|Array|Get(acopy) (Variables|ParanoidEvent|GetSkeletalMeshes) _index)) (.Location (Math|Transform|BreakTransform (Utilities|AddActorOffset (Utilities|Array|Get(acopy) (Variables|ParanoidEvent|GetTeleportLocations) _index)))) 0.0 (select (== (Math|Integer|%(Integer) _index 2) 0) "(R=0.834525,G=1.000000,B=0.000000,A=1.000000)" "(R=0.000000,G=1.000000,B=0.434016,A=1.000000)") 9e+01 3.0))
    (else
      (Rendering|Debug|FlushPersistentDebugLines))))

(event EventInvokeEvent
  (for (_array_element _array_index) (Variables|ParanoidEvent|GetSkeletalMeshes)
    (Variables|Default|SetCurrentActor _array_element)
    (if (not (Class|Actor|WasRecentlyRendered (Variables|Default|GetCurrentActor) 0.016))
      (Transformation|SetActorTransform (Variables|Default|GetCurrentActor) (Utilities|AddActorOffset (Utilities|Array|Get(acopy) (Variables|ParanoidEvent|GetTeleportLocations) _array_index)) false true))))

(fn ConstructionScript
  (|CallParentFunction)
  (Class|ParanoidEvent|UpdateDebugSymbols))