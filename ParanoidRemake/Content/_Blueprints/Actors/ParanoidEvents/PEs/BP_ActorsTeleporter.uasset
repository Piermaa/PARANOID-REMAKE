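; Paranoid event actor that teleports a list of actors to index-matched target transforms when InvokeEvent fires.
; Targets pass through an AddActorOffset helper at unit scale, and the move happens without sweep or any player-visibility check, despite the graph comment.
; The construction script can draw alternating-colored arrows from each actor to its target, while BeginPlay draws spheres at the targets.
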(event EventUpdateDebugSymbols
  (Rendering|Debug|FlushPersistentDebugLines)
  (if (Variables|Default|GetShowDebugElements)
    (for _index (range 0 (- (Utilities|Array|Length (Variables|ParanoidEvent|GetActors)) 1))
      (Rendering|Debug|DrawDebugArrow (Transformation|GetActorLocation (Utilities|Array|Get(acopy) (Variables|ParanoidEvent|GetActors) _index)) (.Location (Math|Transform|BreakTransform (Utilities|AddActorOffset (Utilities|Array|Get(acopy) (Variables|ParanoidEvent|GetTeleportLocations) _index)))) 0.0 (select (== (Math|Integer|%(Integer) _index 2) 0) "(R=0.834525,G=1.000000,B=0.000000,A=1.000000)" "(R=0.000000,G=1.000000,B=0.434016,A=1.000000)") 9e+01 3.0))))

(event EventBeginPlay
  (for _array_element (Variables|ParanoidEvent|GetTeleportLocations)
    (Rendering|Debug|DrawDebugSphere (.Location (Math|Transform|BreakTransform (Utilities|AddActorOffset _array_element))) 1e+01 12 "(R=0.806653,G=0.799631,B=1.000000,A=1.000000)" 1e+02)))

(event EventInvokeEvent
  ;[1 1 1 1 35] Invoke Event
  ;;[1 1 1] Checks if the player sees the skms to move
  (for (_array_element _array_index) (Variables|ParanoidEvent|GetActors)
    (Transformation|SetActorTransform _array_element (Utilities|AddActorOffset (Utilities|Array|Get(acopy) (Variables|ParanoidEvent|GetTeleportLocations) _array_index) "1.000000,1.000000,1.000000") false true)))

(event EventTick
  (params (DeltaSeconds :type Float%20%28single-precision%29))
  (Rendering|Debug|DrawDebugLine "0, 0, 0" "0, 0, 0" "(R=0.000000,G=0.000000,B=0.000000,A=1.000000)" 0.001 0.0))

(fn ConstructionScript
  (|CallParentFunction)
  (Class|ParanoidEvent|UpdateDebugSymbols))