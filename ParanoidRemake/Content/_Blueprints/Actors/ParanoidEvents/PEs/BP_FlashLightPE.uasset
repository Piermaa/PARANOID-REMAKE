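; Paranoid event actor that fires a brief spotlight flash and triggers a flash effect on nearby pawns.
; When invoked, it raises the spotlight to flash intensity, messages overlapping pawns in its sphere through the player post-process interface, then switches the light off after a short delay.
; The construction script applies light color, radius and cone angles, showing the light in the editor only when the debug flag is set, while BeginPlay turns it off.
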(event EventInvokeEvent
  (Rendering|Components|Light|SetIntensity (Variables|Default|GetSpotLight) (Variables|Flash|GetFlash%20Intensity))
  (for _array_element (Collision|GetOverlappingActors (Variables|Default|GetSphere) "/Script/Engine.Pawn" :!class /Script/Engine.PrimitiveComponent)
    (if (Utilities|DoesObjectImplementInterface _array_element "/Game/_Blueprints/BlueprintInterfaces/BPI_PlayerPostProcess.BPI_PlayerPostProcess_C")
      (Class|BPIPlayerPostProcess|FnDispatchFlashEffect(Message) _array_element)))
  (Utilities|FlowControl|Delay 0.1)
  (Rendering|Components|Light|SetIntensity (Variables|Default|GetSpotLight) 0.0))

(event EventBeginPlay
  (|CallParentFunction)
  (Rendering|Components|Light|SetIntensity (Variables|Default|GetSpotLight) 0.0))

(fn ConstructionScript
  (bind _spotlight (Variables|Default|GetSpotLight))
  (Rendering|Components|Light|SetLightColor _spotlight (Variables|Light|GetColor) true)
  (Rendering|Lighting|SetAttenuationRadius _spotlight (Variables|Light|GetRadius))
  (Rendering|Lighting|SetOuterConeAngle _spotlight (Variables|Light|GetOuter%20Cone%20Angle))
  (Rendering|Lighting|SetInnerConeAngle _spotlight (Variables|Light|GetInner%20Cone%20Angle))
  (Rendering|Components|Light|SetIntensity (Variables|Default|GetSpotLight) (Math|Float|SelectFloat (Variables|Flash|GetFlash%20Intensity) 0.0 (Variables|Debugging|GetDebugLights))))