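; BP_DialogueSoundPlayerPE is a paranoid event actor that plays a dialogue line through the player's HUD subtitles when invoked.
; On InvokeEvent it calls the parent event, casts the player controller to PC_FirstPersonController, then fetches the dialogue by its DialogueID row name.
; The result is passed to SetNewDialogue on the HUD's subtitles master widget.
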(event EventInvokeEvent
  (|CallParentFunction)
  (bind _aspc_first_person_controller (Utilities|Casting|CastToPC_FirstPersonController (Game|GetPlayerController 0)))
  (Default|SetNewDialogue (Variables|/Game/_Blueprints/Widgets/WBP_HUD.WBP_HUD_C|GetWBP_SubtitlesMaster (Variables|/Game/_Blueprints/Controller/PC_FirstPersonController.PC_FirstPersonController_C|GetHUD%20Widget _aspc_first_person_controller)) (CallFunction|GetDialogue (Utilities|Struct|BreakDataTableRowHandle (Variables|ParanoidEvent|GetDialogue%20ID)))))

(fn ConstructionScript
  (|CallParentFunction))