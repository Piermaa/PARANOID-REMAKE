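; Paranoid event actor that plays a Level Sequence as a scripted moment when its InvokeEvent fires.
; It creates a sequence player for its LevelSequence at runtime, starts playback and disables input on player 0's controlled pawn.
; A Delay based on the sequence's play length re-enables input afterward, rather than binding to the player's finished event.
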(event EventInvokeEvent
  (bind _returnvalue (Game|GetPlayerController 0))
  (bind _returnvalue_2 (Game|GetPlayerController 0))
  (bind _outactor (Sequencer|Player|CreateLevelSequencePlayer (Variables|ParanoidEvent|GetLevel%20Sequence)))
  (Sequencer|Player|Play (Variables|/Script/LevelSequence.LevelSequenceActor|GetSequencePlayer _outactor) :!class /Script/MovieScene.MovieSceneSequencePlayer)
  (Input|DisableInput (Pawn|GetControlledPawn _returnvalue_2) _returnvalue_2)
  (bind _returnvalue_3 (Animation|GetPlayLength (Variables|/Script/LevelSequence.LevelSequenceActor|GetSequencePlayer _outactor)))
  (Utilities|FlowControl|Delay _returnvalue_3)
  (Input|EnableInput (Pawn|GetControlledPawn _returnvalue) _returnvalue))

(fn ConstructionScript)