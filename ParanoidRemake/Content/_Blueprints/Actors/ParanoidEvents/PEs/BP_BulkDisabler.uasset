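; BP_BulkDisabler is a paranoid event actor that switches off, in bulk, the actors found inside its box volume.
; InvokeEvent, also bound to a debug B key, runs a multi box trace on the Visibility channel at the actor's transform.
; Each hit actor is hidden with collision disabled, and static mesh actors also get their mesh components hidden and made non-colliding.
; The construction script draws the box as a debug preview.
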(event EventUpdateDebugSymbols
  (Rendering|Debug|FlushPersistentDebugLines)
  (Rendering|Debug|DrawDebugBox (Transformation|GetActorLocation) (Variables|ParanoidEvent|GetExtent) "(R=1.000000,G=0.135417,B=0.135417,A=1.000000)" (Transformation|GetActorRotation) 1e+01 1e+01))

(event EventInvokeEvent
  (bind _returnvalue (Transformation|GetActorLocation))
  (bind _outhits (Class|KismetSystemLibrary|BoxTraceMulti _returnvalue _returnvalue (Variables|ParanoidEvent|GetExtent) (Transformation|GetActorRotation) "TraceTypeQuery1" false 0 "ForDuration" true))
  (for _array_element _outhits
    (CallFunction|FSetActive true (.HitActor (Collision|BreakHitResult _array_element)))))

(event Input|KeyboardEvents|DebugKeyB
  (params (Key :type Key%20Structure :default "None") (ActionValue :type Input%20Action%20Value%20Structure))
  (:Pressed
    (Class|ParanoidEventInterface|InvokeEvent)))

(fn ConstructionScript
  (|CallParentFunction)
  (Class|ParanoidEvent|UpdateDebugSymbols))

(fn DrawLines
  (params (Array :type Array%20of%20Actor%20Object%20References) (LineColor :type Linear%20Color%20Structure))
  (for _array_element Array
    (Rendering|Debug|DrawDebugLine (Transformation|GetActorLocation) (Transformation|GetActorLocation _array_element) LineColor 9e+01 0.0))
  (return))

(fn FSetActive
  (params (Disabled? :type Boolean) (Actor :type Actor%20Object%20Reference))
  (bind _returnvalue (Actor|GetComponentsByClass Actor "/Script/Engine.StaticMeshComponent"))
  (LocalVariables|SetP_NewActive Disabled?)
  (Rendering|SetActorHiddenInGame Actor (LocalVariables|GetP_NewActive))
  (Collision|SetActorEnableCollision Actor (not (LocalVariables|GetP_NewActive)))
  (bind _asstatic_mesh_actor (Utilities|Casting|CastToStaticMeshActor Actor))
  (Rendering|SetVisibility (Variables|/Script/Engine.StaticMeshActor|GetStaticMeshComponent _asstatic_mesh_actor) (not (LocalVariables|GetP_NewActive)) true)
  (Collision|SetActorEnableCollision _asstatic_mesh_actor (not (LocalVariables|GetP_NewActive)))
  (for _index (range 0 (- (Utilities|Array|Length _returnvalue) 1))
    (Utilities|IsValid (Utilities|Array|Get(acopy) _returnvalue _index)
      (:Is%20Valid
        (Development|SetHiddeninGame (Utilities|Array|Get(acopy) _returnvalue _index) (LocalVariables|GetP_NewActive) true)
        (Collision|SetCollisionEnabled (Utilities|Array|Get(acopy) _returnvalue _index) (select (not (LocalVariables|GetP_NewActive)) "QueryAndPhysics" "NoCollision"))))))