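; BP_ElevatorButton is an interactable floor button for the elevator in the Escopophobia chapter.
; On BeginPlay it finds its BP_Elevator two levels up the attach-parent chain and caches it as the owner.
; Interacting calls MoveToFloor on that elevator with the button's floor number, which the construction script also shows on a text render.
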(event EventBeginPlay
  (bind _asbp_elevator (Utilities|Casting|CastToBP_Elevator (Actor|GetAttachParentActor (Actor|GetAttachParentActor))))
  (Variables|Default|SetElevatorOwner _asbp_elevator))

(event EventInteract
  (Default|MovetoFloor (Variables|Default|GetElevatorOwner) (Variables|Default|GetFloorNumber)))

(fn ConstructionScript
  (Rendering|Components|TextRender|SetText (Variables|Default|GetTextRender) (Utilities|Text|ToText(Integer) (Variables|Default|GetFloorNumber))))