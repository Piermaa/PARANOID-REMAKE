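; BP_FogTrigger is a box trigger volume in the Escopophobia chapter that thickens the fog while the player is inside it.
; On BeginPlay it finds the level's ExponentialHeightFog actor and draws a temporary debug box showing its bounds.
; Player pawn overlap enables volumetric fog and raises density.
; Leaving disables volumetric fog and sets a hardcoded lower density, without saving the fog's original settings.
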(event OnComponentBeginOverlap(Box)
  (params (OverlappedComponent :type Primitive%20Component%20Object%20Reference) (OtherActor :type Actor%20Object%20Reference) (OtherComp :type Primitive%20Component%20Object%20Reference) (OtherBodyIndex :type Integer) (bFromSweep :type Boolean) (SweepResult :type Hit%20Result%20Structure%20%28by%20ref%29))
  (bind _fog (Variables|Default|GetFog))
  (if (== OtherActor (Game|Player|GetPlayerPawn 0))
    (Class|ExponentialHeightFogComponent|SetVolumetricFog (Variables|/Script/Engine.ExponentialHeightFog|GetComponent _fog) true)
    (Class|ExponentialHeightFogComponent|SetFogDensity (Variables|/Script/Engine.ExponentialHeightFog|GetComponent _fog) 3.0)))

(event OnComponentEndOverlap(Box)
  (params (OverlappedComponent :type Primitive%20Component%20Object%20Reference) (OtherActor :type Actor%20Object%20Reference) (OtherComp :type Primitive%20Component%20Object%20Reference) (OtherBodyIndex :type Integer))
  (bind _fog (Variables|Default|GetFog))
  (if (== OtherActor (Game|Player|GetPlayerPawn 0))
    (Class|ExponentialHeightFogComponent|SetVolumetricFog (Variables|/Script/Engine.ExponentialHeightFog|GetComponent _fog) false)
    (Class|ExponentialHeightFogComponent|SetFogDensity (Variables|/Script/Engine.ExponentialHeightFog|GetComponent _fog) 0.4)))

(event EventBeginPlay
  (Rendering|Debug|DrawDebugBox (Transformation|GetWorldLocation (Variables|Default|GetBox)) (Components|Box|GetScaledBoxExtent (Variables|Default|GetBox)) "(R=0.000000,G=0.859375,B=0.402766,A=1.000000)" "0, 0, 0" 1e+02 0.0)
  (bind _returnvalue (Actor|GetActorOfClass "/Script/Engine.ExponentialHeightFog"))
  (Variables|Default|SetFog _returnvalue))

(fn ConstructionScript)