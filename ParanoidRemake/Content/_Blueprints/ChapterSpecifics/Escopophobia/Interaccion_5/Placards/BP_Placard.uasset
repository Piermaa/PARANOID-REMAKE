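; BP_Placard is a placard in the Escopophobia chapter's fifth interaction that fires radial force impulses at random intervals.
; An external caller initializes it with a start delay plus time and force ranges, then passes delta time to FnTimeElapsed instead of the placard using its own tick.
; When the countdown expires, it fires the RadialForce impulse, then rerolls the next interval and impulse strength.
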(event EventFnTimeElapsed
  (params (DeltaTime :type Float%20%28double-precision%29))
  (bind _random_time_limits (Variables|Default|GetRandom%20Time%20Limits))
  (if (<= (- (Variables|Default|GetTimeRemaining) DeltaTime) 0.0)
    (Class|RadialForceComponent|FireImpulse (Variables|Default|GetRadialForce))
    (Variables|Default|SetTimeRemaining (Math|Random|RandomFloatinRange (.x _random_time_limits) (.y _random_time_limits)))
    (Utilities|MRandomizeStrength)
    (else
      (Variables|Default|SetTimeRemaining (- (Variables|Default|GetTimeRemaining) DeltaTime)))))

(event EventFnInitialize
  (params (StartDelay :type Float%20%28double-precision%29) (RandomTimeLimits :type Vector%202D%20Structure) (RandomForceLimits :type Vector%202D%20Structure))
  (Variables|Default|SetRandom%20Time%20Limits RandomTimeLimits)
  (Variables|Default|SetTimeRemaining (+ (Math|Random|RandomFloatinRange (.x (Variables|Default|GetRandom%20Time%20Limits)) (.y (Variables|Default|GetRandom%20Time%20Limits))) StartDelay))
  (Variables|Default|SetRandom%20Force%20Limits RandomForceLimits)
  (Utilities|MRandomizeStrength))

(fn ConstructionScript)