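; Fog hazard for Escopophobia's fifth interaction that sends the player back to a checkpoint on contact.
; InvokeEvent toggles it, switching the Niagara effect and sphere collision and running one of four timelines, picked by TimelineToUse, to move the fog along a spline.
; On player overlap, it sets a checkpoint offset from the actor's location, teleports via AC_CheckpointsController, then calls Begin and Stop back-to-back, leaving itself inactive.
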(event OnComponentBeginOverlap(Sphere)
  (params (OverlappedComponent :type Primitive%20Component%20Object%20Reference) (OtherActor :type Actor%20Object%20Reference) (OtherComp :type Primitive%20Component%20Object%20Reference) (OtherBodyIndex :type Integer) (bFromSweep :type Boolean) (SweepResult :type Hit%20Result%20Structure%20%28by%20ref%29))
  (bind _returnvalue (Actor|GetComponentbyClass OtherActor "/Game/_Blueprints/ChapterSpecifics/Escopophobia/Interaccion_5/Fog/AC_CheckpointsController.AC_CheckpointsController_C"))
  (if (== OtherActor (Game|Player|GetPlayerPawn 0))
    (Default|UpdateCheckpoint _returnvalue (Utilities|MtoWorldTransform (Variables|A-Fog|GetCheclpoint)))
    (Default|FnTeleporttoCheckpoint _returnvalue)
    (CallFunction|Begin)
    (CallFunction|Stop)
    (Variables|Default|SetIsActive false)))

(event Custom|Begin
  (Collision|SetCollisionProfileName (Variables|Default|GetSphere) "OverlapAll" true :!class /Script/Engine.PrimitiveComponent)
  ;[1 0.7982 0.1085 1 50] Timelines
  (Components|Activation|SetActive (Variables|Default|GetNiagara) true true)
  (switch int (Variables|A-Fog|GetTimelineToUse)
    (:1
      (bind _fogadvance (Timeline|Timeline PlayFromStart)
        (:Update
          (CallFunction|UpdateLocation _fogadvance))))
    (:2
      (bind _fogadvance_2 (Timeline|Timeline_0 PlayFromStart)
        (:Update
          (CallFunction|UpdateLocation _fogadvance_2))))
    (:3
      (bind _fogadvance_3 (Timeline|Timeline_1 PlayFromStart)
        (:Update
          (CallFunction|UpdateLocation _fogadvance_3))))
    (:4
      (bind _fogadvance_4 (Timeline|Timeline_2 PlayFromStart)
        (:Update
          (CallFunction|UpdateLocation _fogadvance_4))))))

(event Custom|Stop
  (Collision|SetCollisionProfileName (Variables|Default|GetSphere) "NoCollision" true :!class /Script/Engine.PrimitiveComponent)
  ;[1 0.7982 0.1085 1 50] Timelines
  (Components|Activation|SetActive (Variables|Default|GetNiagara) false true)
  (switch int (Variables|A-Fog|GetTimelineToUse)
    (:1
      (bind _fogadvance (Timeline|Timeline Stop)
        (:Update
          (CallFunction|UpdateLocation _fogadvance))))
    (:2
      (bind _fogadvance_2 (Timeline|Timeline_0 Stop)
        (:Update
          (CallFunction|UpdateLocation _fogadvance_2))))
    (:3
      (bind _fogadvance_3 (Timeline|Timeline_1 Stop)
        (:Update
          (CallFunction|UpdateLocation _fogadvance_3))))
    (:4
      (bind _fogadvance_4 (Timeline|Timeline_2 Stop)
        (:Update
          (CallFunction|UpdateLocation _fogadvance_4))))))

(event Custom|UpdateLocation
  (params (Alpha :type Float%20%28double-precision%29))
  ;[1 0.7982 0.1085 1 50] Timelines
  (Transformation|SetRelativeLocation (Variables|Default|GetNiagara) (Spline|GetLocationatDistanceAlongSpline (Variables|Default|GetSpline) (Utilities|MGetDistanceonSpline Alpha) "Local") true false))

(event EventInvokeEvent
  (if (Variables|Default|GetIsActive)
    (CallFunction|Stop)
    (Variables|Default|SetIsActive false)
    (else
      (CallFunction|Begin)
      (Variables|Default|SetIsActive true))))

(fn ConstructionScript)