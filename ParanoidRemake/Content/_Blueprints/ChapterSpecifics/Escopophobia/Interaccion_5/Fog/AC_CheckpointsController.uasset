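; Checkpoint controller component for the Escopophobia fog interaction that returns the player to the last stored checkpoint.
; UpdateCheckpoint stores a transform, whose location Teleport treats as an offset from the owning actor's position.
; Teleport locks move and look input, plays a fade widget, then moves the pawn and aligns control rotation before unlocking input.
; FnTeleportToCheckpoint starts this delayed sequence and immediately returns the checkpoint transform.
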(event Custom|Teleport
  (bind _returnvalue (Game|GetPlayerController 0))
  (bind _returnvalue_2 (Game|GetPlayerController 0))
  (bind _currentcheckpoint (Variables|Default|GetCurrentCheckpoint))
  (bind (_location _rotation _scale) (Math|Transform|BreakTransform _currentcheckpoint))
  (Input|SetIgnoreMoveInput _returnvalue_2 true)
  (Input|SetIgnoreLookInput _returnvalue_2 true)
  (bind _returnvalue_3 (UserInterface|CreateWidget "/Game/_Blueprints/Widgets/WBP_FadeIn.WBP_FadeIn_C"))
  (UserInterface|Viewport|AddtoViewport _returnvalue_3 0)
  (Default|FadeinFadeOut _returnvalue_3)
  (Utilities|FlowControl|Delay 1.5)
  (Transformation|SetActorTransform (Game|Player|GetPlayerPawn 0) (Math|Transform|MakeTransform (+ _location (Transformation|GetActorLocation (Components|GetOwner))) _rotation _scale))
  (Pawn|SetControlRotation (Game|GetPlayerController 0) _rotation)
  (Utilities|FlowControl|Delay 0.5)
  (Input|SetIgnoreMoveInput _returnvalue false)
  (Input|SetIgnoreLookInput _returnvalue false))

(event Custom|UpdateCheckpoint
  (params (NewCheckpoint :type Transform))
  (Variables|Default|SetCurrentCheckpoint NewCheckpoint))

(fn FnTeleporttoCheckpoint
  (CallFunction|Teleport)
  (return (Variables|Default|GetCurrentCheckpoint)))