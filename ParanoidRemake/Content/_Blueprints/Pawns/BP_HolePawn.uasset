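; Pawn with a limited look-around camera, which hands control back to the first-person character on interact.
; Look input rotates the camera with inverted Y, then clamps yaw to a half-circle and pitch between the VerticalLimit variable and a fixed upper bound.
; The interact action calls PossesFirstPersonCharacter, whose body is not defined in this graph.
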(event Input|EnhancedActionEvents|EnhancedInputActionIA_Look
  (params (ActionValue :type Vector%202D%20Structure) (ElapsedSeconds :type Float%20%28double-precision%29) (TriggeredSeconds :type Float%20%28double-precision%29) (InputAction :type Input%20Action%20Object%20Reference :default "/Game/Input/Actions/IA_Look.IA_Look"))
  (bind _camera (Variables|Default|GetCamera))
  (bind _camera_2 (Variables|Default|GetCamera))
  (bind _camera_3 (Variables|Default|GetCamera))
  (bind _relativerotation (Variables|/Script/Engine.SceneComponent|GetRelativeRotation _camera))
  (bind _relativerotation_2 (Variables|/Script/Engine.SceneComponent|GetRelativeRotation _camera_3))
  (:Triggered
    (Utilities|FlowControl|Sequence
      (:then_0
        (Transformation|AddRelativeRotation (Variables|Default|GetCamera) (Math|Rotator|MakeRotator 0.0 0.0 (.x ActionValue)) true false)
        (Transformation|SetRelativeRotation (Variables|Default|GetCamera) (Math|Rotator|MakeRotator 0.0 (.pitch _relativerotation) (Math|Float|Clamp(Float) (.yaw _relativerotation) -9e+01 9e+01)) false false))
      (:then_1
        (Transformation|AddRelativeRotation _camera_2 (Math|Rotator|MakeRotator 0.0 (* (.y ActionValue) -1.0) 0.0) true false)
        (Transformation|SetRelativeRotation _camera_2 (Math|Rotator|MakeRotator 0.0 (Math|Float|Clamp(Float) (.pitch _relativerotation_2) (Variables|Default|GetVerticalLimit) 7e+01) (.yaw _relativerotation_2)) false false)))))

(event Input|EnhancedActionEvents|EnhancedInputActionIA_Interact
  (params (ActionValue :type Boolean) (ElapsedSeconds :type Float%20%28double-precision%29) (TriggeredSeconds :type Float%20%28double-precision%29) (InputAction :type Input%20Action%20Object%20Reference :default "/Game/Input/Actions/IA_Interact.IA_Interact"))
  (:Triggered
    (CallFunction|PossesFirstPersonCharacter)))

(fn ConstructionScript
  (|CallParentFunction))