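; Possessable pawn whose camera the player rotates with look input, handing possession back to the first-person character on interact.
; Look input adds relative yaw and inverted pitch to the camera; the horizontal and vertical clamp logic is present but disconnected, so no limits apply here.
; Key add, consume, check and get calls pass straight through to a KeyHolder, so the pawn can act as a key-carrying actor.
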(event Input|EnhancedActionEvents|EnhancedInputActionIA_Look
  (params (ActionValue :type Vector%202D%20Structure) (ElapsedSeconds :type Float%20%28double-precision%29) (TriggeredSeconds :type Float%20%28double-precision%29) (InputAction :type Input%20Action%20Object%20Reference :default "/Game/Input/Actions/IA_Look.IA_Look"))
  (:Triggered
    (Utilities|FlowControl|Sequence
      (:then_0
        (Transformation|AddRelativeRotation (Variables|Default|GetCamera) (Math|Rotator|MakeRotator 0.0 0.0 (.x ActionValue)) true false))
      (:then_1
        (Transformation|AddRelativeRotation (Variables|Default|GetCamera) (Math|Rotator|MakeRotator 0.0 (* (.y ActionValue) -1.0) 0.0) true false)))))

(event Input|EnhancedActionEvents|EnhancedInputActionIA_Interact
  (params (ActionValue :type Boolean) (ElapsedSeconds :type Float%20%28double-precision%29) (TriggeredSeconds :type Float%20%28double-precision%29) (InputAction :type Input%20Action%20Object%20Reference :default "/Game/Input/Actions/IA_Interact.IA_Interact"))
  (:Triggered
    (CallFunction|PossesFirstPersonCharacter)))

(event EventConsumeKeysfromActor
  (params (KeysToConsume :type Array%20of%20Names))
  (Class|KeyHolderComponent|ConsumeKeys (Variables|Default|GetKeyHolder) KeysToConsume))

(event EventAddKeytoActor
  (params (NewKey :type Name :default "None"))
  (Class|KeyHolderComponent|AddKey (Variables|Default|GetKeyHolder) NewKey))

(fn ConstructionScript
  (|CallParentFunction))

(fn ActorHasKeys
  (params (KeysToCheck :type Array%20of%20Names))
  (return (Class|KeyHolderComponent|HasKeys (Variables|Default|GetKeyHolder) KeysToCheck)))

(fn GetKeysfromActor
  (return (Class|KeyHolderComponent|GetHeldKeys (Variables|Default|GetKeyHolder))))