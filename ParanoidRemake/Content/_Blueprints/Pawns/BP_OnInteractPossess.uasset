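; Possessable pawn base that lets player 0 take control of it by interacting and later hand control back to the first-person character.
; Interact caches the player's BP_PlayerCharacter and halts its movement, then has the player controller possess this pawn if CheckIsPossessable returns true.
; CheckIsPossessable simply returns the IsPossessable flag, and PossesFirstPersonCharacter re-possesses the cached character.
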(event Custom|Posses%20First%20Person%20Character
  (Pawn|Possess (Game|GetPlayerController 0) (Variables|Default|GetBP_FirstPersonCharacter)))

(event EventBeginPlay)

(event EventInteract
  (Utilities|FlowControl|Sequence
    (:then_0
      (bind _asbp_player_character (Utilities|Casting|CastToBP_PlayerCharacter (Game|GetPlayerCharacter 0)))
      (Variables|Default|SetBP_FirstPersonCharacter _asbp_player_character)
      (Components|Movement|StopMovementImmediately (Variables|/Script/Engine.Character|GetCharacterMovement _asbp_player_character)))
    (:then_1
      (if (CallFunction|CheckIsPossessable)
        (Pawn|Possess (Game|GetPlayerController 0) self)))))

(fn ConstructionScript)

(fn CheckIsPossessable
  (return (Variables|Default|GetbIsPossessable)))