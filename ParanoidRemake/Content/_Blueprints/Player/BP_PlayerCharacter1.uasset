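; Player character Blueprint that plays surface-aware footstep sounds.
; On BeginPlay it binds to the Footsteps component's delegate; each event, if enabled, line-traces downward from the actor to read the physical material surface.
; RealisticRunningComponent's running-speed check selects walk or run variants for wood, concrete or grass, played as non-spatial 2D sounds.
; The trace's timed debug drawing is left on.
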(event Custom|Play%20Footsteps%20Sound
  (bind _returnvalue (Transformation|GetActorLocation))
  ;[0 0.2372 1] FOOTSTEPS
  (if (Variables|Default|GetFootstepsEnabled)
    (bind (_outhit _returnvalue_2) (Collision|LineTraceByChannel _returnvalue (+ _returnvalue "0.000000,0.000000,-300.000000") "TraceTypeQuery1" false 0 "ForDuration" true "(R=1.000000,G=0.000000,B=0.000000,A=1.000000)" "(R=0.000000,G=1.000000,B=0.000000,A=1.000000)" 2.0))
    (if _returnvalue_2
      (if (Class|RealisticRunningComponent|ReachedRunningSpeed (Variables|Default|GetRealisticRunningComponent))
        (switch Utilities|FlowControl|Switch|SwitchonEPhysicalSurface (Variables|/Script/PhysicsCore.PhysicalMaterial|GetSurfaceType (.PhysMat (Collision|BreakHitResult _outhit)))
          (:SurfaceType1
            (Audio|PlaySound2D "/Game/Audio/SoundPresets/Footsteps/MSP_SFX_Footsteps_Wood_Run.MSP_SFX_Footsteps_Wood_Run" 1.0 1.0 0.0 0 0))
          (:SurfaceType2
            (Audio|PlaySound2D "/Game/Audio/SoundPresets/Footsteps/MSP_SFX_Footsteps_Concrete_Run.MSP_SFX_Footsteps_Concrete_Run" 1.0 1.0 0.0 0 0))
          (:SurfaceType3
            (Audio|PlaySound2D "/Game/Audio/SoundPresets/Footsteps/MSP_SFX_Footsteps_Grass_Run.MSP_SFX_Footsteps_Grass_Run" 1.0 1.0 0.0 0 0)))
        (else
          (switch Utilities|FlowControl|Switch|SwitchonEPhysicalSurface (Variables|/Script/PhysicsCore.PhysicalMaterial|GetSurfaceType (.PhysMat (Collision|BreakHitResult _outhit)))
            (:SurfaceType1
              (Audio|PlaySound2D "/Game/Audio/SoundPresets/Footsteps/MSP_SFX_Footsteps_Wood.MSP_SFX_Footsteps_Wood" 1.0 1.0 0.0 0 0))
            (:SurfaceType2
              (Audio|PlaySound2D "/Game/Audio/SoundPresets/Footsteps/MSP_SFX_Footsteps_Concrete.MSP_SFX_Footsteps_Concrete" 1.0 1.0 0.0 0 0))
            (:SurfaceType3
              (Audio|PlaySound2D "/Game/Audio/SoundPresets/Footsteps/MSP_SFX_Footsteps_Grass.MSP_SFX_Footsteps_Grass" 1.0 1.0 0.0 0 0))))))))

(event EventBeginPlay
  ;[0 0.2372 1] FOOTSTEPS
  (|CallParentFunction)
  (EventDispatchers|BindEventtoOnFootstepsDelegate (Variables|Default|GetFootsteps) (delegate Custom|Play%20Footsteps%20Sound)))

(fn ConstructionScript)