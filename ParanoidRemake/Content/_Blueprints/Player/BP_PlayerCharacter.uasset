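; BP_PlayerCharacter is the player character Blueprint, currently holding a test of surface-dependent sounds, apparently for footsteps.
; Tick runs through a Delay, so roughly twice a second it line-traces downward from the actor on the Visibility channel, with debug drawing.
; The hit physical material's surface type selects a test 2D sound and debug print for Wood or Concrete.
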(event EventBeginPlay)

(event Collision|EventActorBeginOverlap
  (params (OtherActor :type Actor%20Object%20Reference)))

(event EventTick
  (params (DeltaSeconds :type Float%20%28single-precision%29))
  (bind _returnvalue (Transformation|GetActorLocation))
  ;[1 0 0] LAVAME SUCIO DIGO SOLO PRUEBA  ENCARGATE DE IMPLEMENTAR ESTO DONDE SEA HAGAS LOS PASOS
  (Utilities|FlowControl|Delay 0.5)
  (bind _outhit (Collision|LineTraceByChannel _returnvalue (+ _returnvalue "0.000000,0.000000,-150.000000") "TraceTypeQuery1" false 0 "ForDuration" true "(R=1.000000,G=0.000000,B=0.000000,A=1.000000)" "(R=0.000000,G=1.000000,B=0.000000,A=1.000000)" 2.0))
  (switch Utilities|FlowControl|Switch|SwitchonEPhysicalSurface (Variables|/Script/PhysicsCore.PhysicalMaterial|GetSurfaceType (.PhysMat (Collision|BreakHitResult _outhit)))
    (:SurfaceType1
      (Audio|PlaySound2D "/Game/Audio/SoundPresets/MSP_SFX_Test.MSP_SFX_Test" 1.0 1.0 0.0 0 0)
      (Development|PrintString "Madera- Test en -> BP_PlayerCharacter Tick"))
    (:SurfaceType2
      (Audio|PlaySound2D "/Game/Audio/SoundPresets/MSP_SFX_Test2.MSP_SFX_Test2" 1.0 1.0 0.0 0 0)
      (Development|PrintString "Concrete- Test en -> BP_PlayerCharacter Tick"))))

(fn ConstructionScript)