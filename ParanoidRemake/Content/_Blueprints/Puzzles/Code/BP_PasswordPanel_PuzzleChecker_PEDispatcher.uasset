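; Password panel puzzle checker that builds a code from button presses and shows it on a text display.
; Until solved, button codes append to the entry, with -2 clearing it and -1 submitting it to CheckPuzzleSolution.
; The default code's length limits input (one extra character gets through) and sets the dash padding width.
; The default code displays on construction and clear, and "OPEN" on solve, after calling the parent handler.
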(event Custom|ReceivePressedBtn
  (params (ButtonCode :type Integer))
  (if (not (Variables|Default|GetbIsSolved))
    (switch int ButtonCode
      (:Default
        (if (not (> (Utilities|String|Len (Variables|Default|GetCurrentPassword)) (Utilities|String|Len (Variables|Default|GetDefaultPasswordCode))))
          (bind _output_get (Variables|Default|SetCurrentPassword (Utilities|String|Append (Variables|Default|GetCurrentPassword) (Utilities|String|ToString(Integer) ButtonCode))))
          (CallFunction|FUpdateText _output_get)))
      (:-2
        (Variables|Default|SetCurrentPassword "")
        (CallFunction|FUpdateText (Variables|Default|GetDefaultPasswordCode)))
      (:-1
        (CallFunction|CheckPuzzleSolution (Variables|Default|GetCurrentPassword))))))

(event EventOnPuzzleSolved
  (|CallParentFunction)
  (CallFunction|FUpdateText "OPEN"))

(fn ConstructionScript
  (|CallParentFunction)
  (CallFunction|FUpdateText (Variables|Default|GetDefaultPasswordCode)))

(fn FUpdateText
  (params (NewText :type String))
  (LocalVariables|SetTempNewText NewText)
  (for _index (range 0 (- (- (Utilities|String|Len (Variables|Default|GetDefaultPasswordCode)) (Utilities|String|Len NewText)) 1))
    (LocalVariables|SetTempNewText (Utilities|String|Append (LocalVariables|GetTempNewText) "-")))
  (Rendering|Components|TextRender|SetText (Variables|Default|GetPasswordText) (Utilities|Text|ToText(String) (LocalVariables|GetTempNewText))))