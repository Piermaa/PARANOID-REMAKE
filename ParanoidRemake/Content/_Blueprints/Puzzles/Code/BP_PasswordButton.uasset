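; BP_PasswordButton is a single key of a password puzzle panel, either a digit or one of two special keys labeled A and B.
; On BeginPlay it caches its attach parent as the puzzle-checker panel, and on Interact it passes its ButtonNumber to that panel.
; The construction script derives the key's text and color from ButtonNumber, with negative values marking the special keys.
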(event EventBeginPlay
  (bind _asbp_password_panel_puzzle_checker_pedispatcher (Utilities|Casting|CastToBP_PasswordPanel_PuzzleChecker_PEDispatcher (Actor|GetAttachParentActor)))
  (Variables|Default|SetPasswordPanel _asbp_password_panel_puzzle_checker_pedispatcher))

(event EventInteract
  (bind _passwordpanel (Variables|Default|GetPasswordPanel)
    (:then
      (Default|ReceivePressedBtn _passwordpanel (Variables|Default|GetButtonNumber)))
    (:else)))

(fn ConstructionScript
  (Rendering|Components|TextRender|SetText (Variables|Default|GetTextRender) (select (>= (Variables|Default|GetButtonNumber) 0) (Utilities|Text|ToText(Integer) (Variables|Default|GetButtonNumber)) (select (== (Variables|Default|GetButtonNumber) -2) (Utilities|Text|MakeLiteralText "B") (Utilities|Text|MakeLiteralText "A"))))
  (Rendering|Components|TextRender|SetTextRenderColor (Variables|Default|GetTextRender) (select (>= (Variables|Default|GetButtonNumber) 0) (Class|KismetMathLibrary|LinearColortoRGBE "(R=0.000000,G=0.000000,B=0.000000,A=1.000000)") (select (== (Variables|Default|GetButtonNumber) -2) (Class|KismetMathLibrary|LinearColortoRGBE "(R=0.166667,G=0.005838,B=0.000000,A=1.000000)") (Class|KismetMathLibrary|LinearColortoRGBE "(R=0.000000,G=0.286458,B=0.128676,A=1.000000)")))))