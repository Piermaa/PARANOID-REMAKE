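; Interactable poster stand for a poster puzzle, holding a swappable poster image and its index.
; An external puzzle checker is assigned with the stand's index at initialization, and interacting reports that index to it.
; Selection fades the spotlight in or out through a timeline.
; New posters set a texture parameter on a dynamic material created at construction, while Tick displays the current poster index as text.
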(event Custom|SetNewPoster
  (params (Texture :type Texture%20Object%20Reference) (PosterIndex :type Integer))
  (Rendering|Material|SetTextureParameterValue (Variables|Default|GetDynamicPosterMaterial) "PosterTexture" Texture)
  (Variables|Default|SetPosterTexture Texture)
  (Variables|Default|SetPoster%20Index PosterIndex))

(event Custom|ToggleSelected
  (params (NowSelected :type Boolean))
  (if NowSelected
    (bind _newtrack_0 (Timeline|Timeline PlayFromStart)
      (:Update
        (Rendering|Components|Light|SetIntensity (Variables|Default|GetSpotLight) (Math|Float|Lerp 0.0 (Variables|Default|GetIntensity) _newtrack_0))))
    (else
      (Timeline|Timeline ReverseFromEnd))))

(event EventBeginPlay
  (Variables|Default|SetIntensity (Variables|/Script/Engine.LightComponentBase|GetIntensity (Variables|Default|GetSpotLight)))
  (CallFunction|ToggleSelected false)
  (Rendering|Material|SetMaterial (Variables|Default|GetStand) 0 (Variables|Default|GetMaterial)))

(event EventTick
  (params (DeltaSeconds :type Float%20%28single-precision%29))
  (Rendering|Components|TextRender|SetText (Variables|Default|GetTextRender) (Utilities|Text|ToText(Integer) (Variables|Default|GetPoster%20Index))))

(event EventInteract
  (Default|SelectPoster (Variables|Default|GetPuzzle%20Checker) (Variables|Default|GetIndex)))

(fn ConstructionScript
  (bind _poster (Variables|Default|GetPoster))
  (Rendering|Material|SetMaterial (Variables|Default|GetStand) 0 (Variables|Default|GetMaterial))
  (Variables|Default|GetDynamicPosterMaterial
    (:then)
    (:else
      (bind _returnvalue (Rendering|Material|CreateDynamicMaterialInstance _poster 0 (Rendering|Material|GetMaterial _poster 0) "None" :!class /Script/Engine.PrimitiveComponent))
      (Variables|Default|SetDynamicPosterMaterial _returnvalue)
      (Rendering|Material|SetMaterial (Variables|Default|GetPoster) 0 _returnvalue))))

(fn FInitialize
  (params (Index :type Integer) (PuzzleChecker :type BP%20Posters%20Puzzle%20Checker%20PE%20Invoker%20Object%20Reference))
  (Variables|Default|SetIndex Index)
  (Variables|Default|SetPuzzle%20Checker PuzzleChecker)
  (Variables|Default|SetPoster%20Index Index))