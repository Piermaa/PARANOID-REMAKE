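; Poster-swapping puzzle checker, where the player selects two stands to exchange their posters.
; The construction script fills five child-actor stands with textures from the default order and registers itself with each.
; The first selection highlights a stand; the second swaps texture and index, then passes the concatenated one-based indices as a password to the inherited solution check.
; On solve it calls the parent handler and prints a debug string.
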(event Custom|SelectPoster
  (params (Index :type Integer))
  (if (== (Variables|Default|GetCurrentlySelectedPoster) -1)
    (Default|ToggleSelected (Utilities|Array|Get(acopy) (Variables|Default|GetPosterStands) Index) true)
    (Variables|Default|SetCurrentlySelectedPoster Index)
    (else
      (Default|ToggleSelected (Utilities|Array|Get(acopy) (Variables|Default|GetPosterStands) (Variables|Default|GetCurrentlySelectedPoster)) false)
      (CallFunction|FSwapPosters (Variables|Default|GetCurrentlySelectedPoster) Index)
      (Variables|Default|SetCurrentlySelectedPoster -1)
      (CallFunction|CheckPuzzleSolution (CallFunction|FGetCurrentPassword)))))

(event EventOnPuzzleSolved
  (|CallParentFunction)
  (Development|PrintString "sexo"))

(fn ConstructionScript
  (|CallParentFunction)
  (for (_array_element _array_index) (Variables|Default|GetPuzzleDefaultOrder)
    (bind _asbp_poster_stand (Utilities|Casting|CastToBP_PosterStand (Variables|/Script/Engine.ChildActorComponent|GetChildActor (Utilities|Select :Index _array_index :Option%200 (Variables|Default|GetChildActor) :Option%201 (Variables|Default|GetChildActor1) :Option%202 (Variables|Default|GetChildActor2) :Option%203 (Variables|Default|GetChildActor3) :Option%204 (Variables|Default|GetChildActor4)))))
    (Default|SetNewPoster _asbp_poster_stand _array_element)
    (Default|FInitialize _asbp_poster_stand _array_index self)
    (Utilities|Array|SetArrayElem (Variables|Default|GetPosterStands) _array_index _asbp_poster_stand true)))

(fn FSwapPosters
  (params (From :type Integer) (To :type Integer))
  (bind _posterstands (Variables|Default|GetPosterStands))
  (bind _posterstands_2 (Variables|Default|GetPosterStands))
  (bind _output (Utilities|Array|Get(acopy) _posterstands To))
  (bind _output_2 (Utilities|Array|Get(acopy) _posterstands_2 From))
  (LocalVariables|SetTempPoster (Variables|/Game/_Blueprints/Puzzles/Posters/BP_PosterStand.BP_PosterStand_C|GetPosterTexture _output))
  (LocalVariables|SetTempIndex (Variables|/Game/_Blueprints/Puzzles/Posters/BP_PosterStand.BP_PosterStand_C|GetPoster%20Index _output))
  (Default|SetNewPoster _output (Variables|/Game/_Blueprints/Puzzles/Posters/BP_PosterStand.BP_PosterStand_C|GetPosterTexture _output_2) (Variables|/Game/_Blueprints/Puzzles/Posters/BP_PosterStand.BP_PosterStand_C|GetPoster%20Index _output_2))
  (Default|SetNewPoster _output_2 (LocalVariables|GetTempPoster) (LocalVariables|GetTempIndex)))

(fn FGetCurrentPassword
  (for _array_element (Variables|Default|GetPosterStands)
    (LocalVariables|SetTempPassword (Utilities|String|Append (LocalVariables|GetTempPassword) (Utilities|String|ToString(Integer) (+ (Variables|/Game/_Blueprints/Puzzles/Posters/BP_PosterStand.BP_PosterStand_C|GetPoster%20Index _array_element) 1)))))
  (return (LocalVariables|GetTempPassword)))