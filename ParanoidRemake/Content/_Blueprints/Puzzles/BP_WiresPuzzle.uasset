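; Wire puzzle manager that penalizes the player for hitting hanging wires and resets them on failure.
; On BeginPlay it binds to every BP_HangingWire's hit event; lost lives deepen the player camera's vignette through a timeline.
; When lives run out, it restores HP and vignette, locks input, fades the screen and moves the player to a respawn transform.
; A trigger box, placed by the construction script, clears the vignette when the player enters.
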(event OnComponentBeginOverlap(ClearVignette)
  (params (OverlappedComponent :type Primitive%20Component%20Object%20Reference) (OtherActor :type Actor%20Object%20Reference) (OtherComp :type Primitive%20Component%20Object%20Reference) (OtherBodyIndex :type Integer) (bFromSweep :type Boolean) (SweepResult :type Hit%20Result%20Structure%20%28by%20ref%29))
  (if (== OtherActor (Game|Player|GetPlayerPawn 0))
    (Utilities|MSetVignette 0.4)))

(event Custom|LooseLife
  (bind _camera (Variables|Default|GetCamera))
  (bind _postprocesssettings (Variables|/Script/Engine.CameraComponent|GetPostProcessSettings _camera))
  (bind _result (Math|Integer|DecrementInt (Variables|Default|GetCurrentHP))
    (:%20%20
      (if (< _result 0)
        (CallFunction|Death)
        (else
          (bind _newtrack_0 (Timeline|Timeline PlayFromStart)
            (:Update
              (Utilities|Struct|SetmembersinPostProcessSettings _postprocesssettings (Math|Float|Lerp (Utilities|Struct|BreakPostProcessSettings _postprocesssettings) (+ (* 0.5 (- (Variables|Default|GetTotalHPs) (Variables|Default|GetCurrentHP))) 0.4) _newtrack_0)))))))))

(event Custom|Death
  (bind _returnvalue (Game|GetPlayerController 0))
  (bind _returnvalue_2 (Game|GetPlayerController 0))
  (bind _newplayerlocation (Variables|Default|GetNewPlayerLocation))
  (bind (_location _rotation _scale) (Math|Transform|BreakTransform _newplayerlocation))
  (Variables|Default|SetCurrentHP (Variables|Default|GetTotalHPs))
  (Utilities|MSetVignette 0.4)
  (Input|SetIgnoreMoveInput _returnvalue_2 true)
  (Input|SetIgnoreLookInput _returnvalue_2 true)
  (bind _returnvalue_3 (UserInterface|CreateWidget "/Game/_Blueprints/Widgets/WBP_FadeIn.WBP_FadeIn_C"))
  (UserInterface|Viewport|AddtoViewport _returnvalue_3 0)
  (Default|FadeinFadeOut _returnvalue_3)
  (Utilities|FlowControl|Delay 1.5)
  (Transformation|SetActorTransform (Game|Player|GetPlayerPawn 0) (Math|Transform|MakeTransform (+ _location (Transformation|GetActorLocation)) _rotation _scale))
  (Pawn|SetControlRotation (Game|GetPlayerController 0) _rotation)
  (Utilities|FlowControl|Delay 0.5)
  (Input|SetIgnoreMoveInput _returnvalue false)
  (Input|SetIgnoreLookInput _returnvalue false))

(event EventBeginPlay
  (Variables|Default|SetCamera (Actor|GetComponentbyClass (Game|Player|GetPlayerPawn 0) "/Script/Engine.CameraComponent"))
  (bind _outactors (Actor|GetAllActorsOfClass "/Game/_Blueprints/Wire/BP_HangingWire.BP_HangingWire_C"))
  (for _array_element _outactors
    (EventDispatchers|BindEventtoOnPlayerHit _array_element (EventDispatchers|CreateEvent :!event Custom|LooseLife))))

(fn ConstructionScript
  (bind _boxlocation (Variables|Default|GetBoxLocation))
  (bind (_location _rotation _scale) (Math|Transform|BreakTransform _boxlocation))
  (Transformation|SetWorldTransform (Variables|Default|GetClear%20Vignette) (Math|Transform|MakeTransform (+ _location (.Location (Math|Transform|BreakTransform (Transformation|GetActorTransform)))) _rotation _scale) false false))