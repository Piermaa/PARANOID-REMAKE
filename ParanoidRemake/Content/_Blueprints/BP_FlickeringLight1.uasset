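; Flickering point light actor that animates its intensity from BeginPlay.
; A timeline track blends between low and high flicker intensities, scaled by brightness and a scale factor, and updates the light on each timeline tick.
; The construction script applies the configurable color and attenuation radius to the light.
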(event EventBeginPlay
  (bind _newtrack_0 (Timeline|Timeline_0 Play)
    (:Update
      (Rendering|Components|Light|SetIntensity (Variables|Default|GetPointLight1) (* (* (Variables|Default|GetLightBrightness) (Variables|Default|GetLightScaleIntensity)) (Math|Float|Lerp (Variables|Default|GetFlickerIntensityLow) (Variables|Default|GetFlickerIntensityHigh) _newtrack_0))))))

(fn ConstructionScript
  (bind _pointlight1 (Variables|Default|GetPointLight1))
  (Rendering|Components|Light|SetLightColor _pointlight1 (Variables|Default|GetColor) true)
  (Rendering|Lighting|SetAttenuationRadius _pointlight1 (Variables|Default|GetRadius)))